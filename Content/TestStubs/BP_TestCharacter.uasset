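; BP_TestCharacter is a test character with axis-driven movement and a camera-aimed laser interaction.
; Space traces along the VR camera's forward vector with persistent debug drawing, sends LazerInteractMessage to the hit actor and plays a shot sound at the character.
; MoveForward and MoveRight add movement input relative to control-rotation yaw only.
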(event Input|AxisEvents|InputAxisMoveForward
  (params (AxisValue :type Float%20%28single-precision%29))
  ;[1 1 1] Movement
  (Pawn|Input|AddMovementInput (Math|Vector|GetForwardVector (Math|Rotator|MakeRotator 0.0 0.0 (.Yaw (Math|Rotator|BreakRotator (Pawn|GetControlRotation :!class /Script/Engine.Pawn))))) AxisValue false))

(event Input|AxisEvents|InputAxisMoveRight
  (params (AxisValue :type Float%20%28single-precision%29))
  ;[1 1 1] Movement
  (Pawn|Input|AddMovementInput (Math|Vector|GetRightVector (Math|Rotator|MakeRotator 0.0 0.0 (.Yaw (Math|Rotator|BreakRotator (Pawn|GetControlRotation :!class /Script/Engine.Pawn))))) AxisValue false))

(event Input|KeyboardEvents|SpaceBar
  (params (Key :type Key%20Structure :default "None"))
  ;[1 1 1] Raycast
  (:Pressed
    (bind (_location _forward_vector) (CallFunction|GetPlayerVRCameraProperties))
    (bind (_outhit _returnvalue) (Collision|LineTraceByChannel _location (+ _location (* _forward_vector 1000)) "TraceTypeQuery1" false 0 "Persistent"))
    (if _returnvalue
      (Class|BPIInteractable|LazerInteract(Message) (.HitActor (Collision|BreakHitResult _outhit)))
      (Audio|SpawnSoundatLocation "/Game/Audio/SoundWaves/Effect/SW_TechShot.SW_TechShot" (Transformation|GetActorLocation) "0, 0, 0" 1.0 1.0 0.0 0 0))))

(fn ConstructionScript)