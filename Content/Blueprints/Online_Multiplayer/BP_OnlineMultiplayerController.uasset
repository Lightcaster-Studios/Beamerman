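; Player controller for online Beamerman matches that handles pawn allocation, game start and per-player UI.
; AllocatePlayer spawns and possesses one of four pawn classes by PlayerIndex at matching PlayerStarts, registering it with the game mode.
; Enter starts the game through the game mode once two players are alive.
; Events drive loading, countdown, HUD, input unfreeze with music, and a paused victory screen fed by game-state player records.
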(event Custom|ShowCountdown
  ;[0.3316 0.29 1] Countdown
  (bind _returnvalue (UserInterface|CreateWidget "/Game/UI/OnlineMultiplayer/CountdownWidget.CountdownWidget_C"))
  (UserInterface|Viewport|AddtoViewport _returnvalue 0))

(event Custom|Unfreeze
  ;[0.3316 0.29 1] Countdown
  (Input|EnableInput (Pawn|GetControlledPawn) self)
  (bind _aspersistent_game_instance (Utilities|Casting|CastToPersistentGameInstance (Game|GetGameInstance)))
  (Default|PlayGameMusic _aspersistent_game_instance))

(event Custom|Open%20Victory%20UI
  ;[0.2042 0.2973 1] UI
  (Viewport|RemoveAllWidgets)
  (Game|SetGamePaused true)
  (Variables|/Script/Engine.PlayerController|SetbShowMouseCursor self true)
  (Input|DisableInput self)
  (bind _aspersistent_game_instance (Utilities|Casting|CastToPersistentGameInstance (Game|GetGameInstance)))
  (Default|PlayEndGameAudio _aspersistent_game_instance)
  (bind _asbp_multiplayer_game_state (Utilities|Casting|CastToBP_MultiplayerGameState (Game|GetGameState)))
  (bind _returnvalue (UserInterface|CreateWidget "/Game/UI/EndGameVictory/UI_Victory.UI_Victory_C" self (Variables|/Game/Blueprints/Online_Multiplayer/BP_MultiplayerGameState.BP_MultiplayerGameState_C|GetPlayerRecords _asbp_multiplayer_game_state)))
  (bind _output_get (Variables|UI|SetVictoryWidgetRef _returnvalue))
  (Variables|/Game/UI/EndGameVictory/UI_Victory.UI_Victory_C|SetCurrentLevelName _output_get "LobbyMap")
  (UserInterface|Animation|PlayAnimation (Variables|UI|GetVictoryWidgetRef) (Variables|/Game/UI/EndGameVictory/UI_Victory.UI_Victory_C|GetSlide (Variables|UI|GetVictoryWidgetRef)) 0.0 1 "Forward" 1.0 false)
  (UserInterface|Viewport|AddtoViewport (Variables|UI|GetVictoryWidgetRef) 0))

(event Custom|Remove%20Loading%20Screen
  ;[1 0.06197 0.1516] Events for showing initialize game loading screen
  (Widget|RemovefromParent (Variables|UI|GetLoading%20Screen)))

(event Custom|OnlineMultiplayerGameHUD
  ;[0.2042 0.2973 1] UI
  (bind _returnvalue (UserInterface|CreateWidget "/Game/UI/HUD/OnlineMultiplayerGameWidgetHUD.OnlineMultiplayerGameWidgetHUD_C"))
  (UserInterface|Viewport|AddtoViewport _returnvalue 0))

(event Custom|Show%20Loading%20Screen
  ;[1 0.06197 0.1516] Events for showing initialize game loading screen
  (bind _returnvalue (UserInterface|CreateWidget "/Game/UI/OnlineMultiplayer/LoadingSettingUpMap.LoadingSettingUpMap_C" self))
  (bind _output_get (Variables|UI|SetLoading%20Screen _returnvalue))
  (UserInterface|Viewport|AddtoViewport _output_get 0))

(event EventBeginPlay
  (bind _asbp_beamerman_multi_player (Utilities|Casting|CastToBP_BeamermanMultiPlayer (Pawn|GetControlledPawn)))
  (Rendering|ToggleVisibility (Variables|/Game/Blueprints/Player/BP_BeamermanMultiPlayer.BP_BeamermanMultiPlayer_C|GetIndicator _asbp_beamerman_multi_player) false)
  (bind _asbp_online_multiplayer_game_mode (Utilities|Casting|CastToBP_OnlineMultiplayerGameMode (Game|GetGameMode)))
  (Variables|Default|SetOnline%20Multiplayer%20Game%20Mode _asbp_online_multiplayer_game_mode))

(event EventAllocatePlayer
  ;[0.1818 0.2017 1] Allocate Player
  (bind _outactors (Actor|GetAllActorsOfClass "/Script/Engine.PlayerStart"))
  (Variables|Default|SetPlayerStart _outactors)
  (switch int (Variables|Default|GetPlayerIndex)
    (:0
      (bind _returnvalue (Game|SpawnActorfromClass "/Game/Blueprints/Online_Multiplayer/BP_Multiplayer_1.BP_Multiplayer_1_C" (Transformation|GetActorTransform (Utilities|Array|Get(acopy) (Variables|Default|GetPlayerStart))) "Undefined" 0 0 0))
      (Pawn|Possess _returnvalue)
      (bind _asbp_beamerman_multi_player (Utilities|Casting|CastToBP_BeamermanMultiPlayer (Pawn|GetControlledPawn)))
      (bind _output_get (Variables|/Game/Blueprints/Player/BP_BeamermanMultiPlayer.BP_BeamermanMultiPlayer_C|SetPlayerID _asbp_beamerman_multi_player (Variables|Default|GetPlayerIndex)))
      (Utilities|Map|Add (Variables|/Game/Blueprints/Online_Multiplayer/BP_OnlineMultiplayerGameMode.BP_OnlineMultiplayerGameMode_C|GetPlayerIndexToPlayerRef (Variables|Default|GetOnline%20Multiplayer%20Game%20Mode)) _output_get _asbp_beamerman_multi_player))
    (:1
      (bind _returnvalue_2 (Game|SpawnActorfromClass "/Game/Blueprints/Online_Multiplayer/BP_Multiplayer_2.BP_Multiplayer_2_C" (Transformation|GetActorTransform (Utilities|Array|Get(acopy) (Variables|Default|GetPlayerStart) 1)) "Undefined" 0 0 0))
      (Pawn|Possess _returnvalue_2)
      (CallFunction|ShowLoadingScreen)
      (bind _asbp_beamerman_multi_player_2 (Utilities|Casting|CastToBP_BeamermanMultiPlayer (Pawn|GetControlledPawn)))
      (bind _output_get_2 (Variables|/Game/Blueprints/Player/BP_BeamermanMultiPlayer.BP_BeamermanMultiPlayer_C|SetPlayerID _asbp_beamerman_multi_player_2 (Variables|Default|GetPlayerIndex)))
      (Utilities|Map|Add (Variables|/Game/Blueprints/Online_Multiplayer/BP_OnlineMultiplayerGameMode.BP_OnlineMultiplayerGameMode_C|GetPlayerIndexToPlayerRef (Variables|Default|GetOnline%20Multiplayer%20Game%20Mode)) _output_get_2 _asbp_beamerman_multi_player_2))
    (:2
      (bind _returnvalue_3 (Game|SpawnActorfromClass "/Game/Blueprints/Online_Multiplayer/BP_Multiplayer_3.BP_Multiplayer_3_C" (Transformation|GetActorTransform (Utilities|Array|Get(acopy) (Variables|Default|GetPlayerStart) 2)) "Undefined" 0 0 0))
      (Pawn|Possess _returnvalue_3)
      (bind _asbp_beamerman_multi_player_3 (Utilities|Casting|CastToBP_BeamermanMultiPlayer (Pawn|GetControlledPawn)))
      (bind _output_get_3 (Variables|/Game/Blueprints/Player/BP_BeamermanMultiPlayer.BP_BeamermanMultiPlayer_C|SetPlayerID _asbp_beamerman_multi_player_3 (Variables|Default|GetPlayerIndex)))
      (Utilities|Map|Add (Variables|/Game/Blueprints/Online_Multiplayer/BP_OnlineMultiplayerGameMode.BP_OnlineMultiplayerGameMode_C|GetPlayerIndexToPlayerRef (Variables|Default|GetOnline%20Multiplayer%20Game%20Mode)) _output_get_3 _asbp_beamerman_multi_player_3))
    (:3
      (bind _returnvalue_4 (Game|SpawnActorfromClass "/Game/Blueprints/Online_Multiplayer/BP_Multiplayer_4.BP_Multiplayer_4_C" (Transformation|GetActorTransform (Utilities|Array|Get(acopy) (Variables|Default|GetPlayerStart) 3)) "Undefined" 0 0 0))
      (Pawn|Possess _returnvalue_4)
      (bind _asbp_beamerman_multi_player_4 (Utilities|Casting|CastToBP_BeamermanMultiPlayer (Pawn|GetControlledPawn)))
      (bind _output_get_4 (Variables|/Game/Blueprints/Player/BP_BeamermanMultiPlayer.BP_BeamermanMultiPlayer_C|SetPlayerID _asbp_beamerman_multi_player_4 (Variables|Default|GetPlayerIndex)))
      (Utilities|Map|Add (Variables|/Game/Blueprints/Online_Multiplayer/BP_OnlineMultiplayerGameMode.BP_OnlineMultiplayerGameMode_C|GetPlayerIndexToPlayerRef (Variables|Default|GetOnline%20Multiplayer%20Game%20Mode)) _output_get_4 _asbp_beamerman_multi_player_4))))

(event Input|KeyboardEvents|Enter
  (params (Key :type Key%20Structure :default "None"))
  (bind _online_multiplayer_game_mode (Variables|Default|GetOnline%20Multiplayer%20Game%20Mode))
  ;[0.3316 0.29 1] Countdown
  (:Pressed
    (if (>= (Utilities|Set|Length (Variables|/Game/Blueprints/Online_Multiplayer/BP_OnlineMultiplayerGameMode.BP_OnlineMultiplayerGameMode_C|GetAlivePlayers _online_multiplayer_game_mode)) 2)
      (Default|StartGame _online_multiplayer_game_mode))))

(fn ConstructionScript)

(fn SetPlayerAppearance
  (params (PlayerIndex :type Integer) (Player :type BP%20Beamerman%20Multi%20Player%20Object%20Reference))
  (bind _mesh (Variables|/Script/Engine.Character|GetMesh Player))
  (Variables|/Game/Blueprints/Player/BP_BeamermanMultiPlayer.BP_BeamermanMultiPlayer_C|SetDroneMaterial Player (Utilities|Array|Get(acopy) (Variables|PlayerAppearance|GetPlayerDroneMaterials) PlayerIndex))
  (Variables|/Game/Blueprints/Player/BP_BeamermanMultiPlayer.BP_BeamermanMultiPlayer_C|SetLazerMaterial Player (Utilities|Array|Get(acopy) (Variables|PlayerAppearance|GetPlayerLazerMaterials) PlayerIndex))
  (Class|SkinnedMeshComponent|SetSkeletalMesh _mesh (Utilities|Array|Get(acopy) (Variables|PlayerAppearance|GetPlayerSkeletalMeshes) PlayerIndex) true)
  (Rendering|Material|SetMaterial _mesh 1 (Utilities|Array|Get(acopy) (Variables|PlayerAppearance|GetPlayerMaterials) PlayerIndex)))

(fn OnRepPlayerIndex)