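; Game mode for online Beamerman matches of up to four players, running from waiting screen to last-player-standing victory.
; PostLogin registers each pre-start joiner with an index; StartGame runs countdown, score setup, unfreeze, HUD and match timer.
; Each player's capsule gets its own collision channel, mapped in the persistent game instance.
; Tick watches for one survivor, then publishes death records to the game state and opens victory UI.
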(event Custom|Start%20Game
  (if (not (Variables|Default|GetOnline%20Multiplayer%20Game%20Started?))
    (for _array_element (Variables|Default|GetOnline%20Multiplayer%20Controllers)
      (Default|ShowCountdown _array_element)
      (Widget|RemovefromParent (stale EventBeginPlay _returnvalue)))
    (Variables|Default|SetOnline%20Multiplayer%20Game%20Started? true)
    (CallFunction|CreateScore)
    (Utilities|FlowControl|Delay 3.0)
    (CallFunction|Unfreeze)
    (CallFunction|Collision)
    (CallFunction|GameHUD)))

(event Custom|Unfreeze
  ;[1 1 1] Unfreeze
  (for _array_element (Variables|Default|GetOnline%20Multiplayer%20Controllers)
    (Default|Unfreeze _array_element))
  (Variables|/Game/Blueprints/Online_Multiplayer/BP_MultiplayerGameState.BP_MultiplayerGameState_C|SetCurrentTime (Variables|Default|GetMyGameState) (Variables|Default|GetMatchTime))
  (Utilities|Time|SetTimerbyEvent (delegate Custom|Count) 1.0 true))

(event Custom|Count
  ;[1 1 1] Unfreeze
  (Math|Integer|DecrementInt (Variables|/Game/Blueprints/Online_Multiplayer/BP_MultiplayerGameState.BP_MultiplayerGameState_C|GetCurrentTime (Variables|Default|GetMyGameState))))

(event Custom|Collision
  ;[1 1 1] Unfreeze
  (CallFunction|SetPlayerCollisions)
  (bind _aspersistent_game_instance (Utilities|Casting|CastToPersistentGameInstance (Game|GetGameInstance)))
  (Variables|/Game/PersistentGameInstance.PersistentGameInstance_C|SetAllOnlinePlayers _aspersistent_game_instance (Variables|Default|GetOnline%20Multi%20Player%20Objects)))

(event Custom|GameHUD
  (for _array_element (Variables|Default|GetOnline%20Multiplayer%20Controllers)
    (Default|OnlineMultiplayerGameHUD _array_element)))

(event Custom|Set%20Game%20State
  (Variables|/Game/Blueprints/Online_Multiplayer/BP_MultiplayerGameState.BP_MultiplayerGameState_C|SetPlayers (Variables|Default|GetMyGameState) (Variables|Default|GetOnline%20Multi%20Player%20Objects)))

(event Custom|Victory
  ;[0.2399 0.156 1] Add last alive guy to the player records
  (bind _result (Utilities|Set|ToArray (Variables|Default|GetAlivePlayers)))
  (CallFunction|RegisterPlayerDeathinGameMode (.Value (Utilities|Map|Find (Variables|Default|GetPlayer%20Index%20to%20Multi%20Player%20Object%20Ref) (Utilities|Array|Get(acopy) _result))))
  (Variables|/Game/Blueprints/Online_Multiplayer/BP_MultiplayerGameState.BP_MultiplayerGameState_C|SetPlayer%20Death%20Records (Variables|Default|GetMyGameState) (Variables|Default|GetPlayerRecords))
  (Utilities|FlowControl|Delay 3.0)
  (for _array_element (Variables|Default|GetOnline%20Multiplayer%20Controllers)
    (Default|OpenVictoryUI _array_element)))

(event Custom|Create%20Score
  (for _array_element (Variables|Default|GetOnline%20Multi%20Player%20Objects)
    (Default|CreateScoreTracker _array_element)))

(event EventBeginPlay
  (bind _asbp_multiplayer_game_state (Utilities|Casting|CastToBP_MultiplayerGameState (Game|GetGameState)))
  (Variables|Default|SetMyGameState _asbp_multiplayer_game_state)
  (Variables|/Script/Engine.PlayerController|SetbShowMouseCursor (Game|GetPlayerController 0) false)
  (bind _returnvalue (UserInterface|CreateWidget "/Game/UI/OnlineMultiplayer/WaitingServerStart.WaitingServerStart_C"))
  (UserInterface|Viewport|AddtoViewport _returnvalue 0)
  (bind _aspersistent_game_instance (Utilities|Casting|CastToPersistentGameInstance (Game|GetGameInstance)))
  (Variables|Default|SetPersistentGameInstanceRef _aspersistent_game_instance))

(event EventTick
  (params (DeltaSeconds :type Float%20%28single-precision%29))
  ;[0.2042 0.2973 1] Constantly check if there is only 1 player left, if so, show end game  screen for every single player
  (if (Math|Boolean|ANDBoolean (Variables|Default|GetOnline%20Multiplayer%20Game%20Started?) (== (Utilities|Set|Length (Variables|Default|GetAlivePlayers)) 1) (Variables|Default|GetOnline%20Multiplayer%20Game%20Not%20Ended))
    (Variables|Default|SetOnline%20Multiplayer%20Game%20Not%20Ended false)
    (CallFunction|Victory)))

(event EventPostLogin
  (params (NewPlayer :type Player%20Controller%20Object%20Reference))
  (bind _clientindex (Variables|Default|GetClientIndex))
  ;[0.1292 0.2269 1] Client Joining Server
  (Audio|PlaySound2D "/Game/Audio/SFX/start-game-sfx.start-game-sfx" 1.0 1.0 0.0 0 0)
  (if (not (Variables|Default|GetOnline%20Multiplayer%20Game%20Started?))
    (bind _asbp_online_multiplayer_controller (Utilities|Casting|CastToBP_OnlineMultiplayerController NewPlayer))
    (if (not (Utilities|Array|ContainsItem (Variables|Default|GetOnline%20Multiplayer%20Controllers) _asbp_online_multiplayer_controller))
      (Utilities|Array|Add (Variables|Default|GetOnline%20Multiplayer%20Controllers) _asbp_online_multiplayer_controller)
      (bind _output_get (Variables|Default|SetCurrentPlayer _asbp_online_multiplayer_controller))
      (Variables|/Game/Blueprints/Online_Multiplayer/BP_OnlineMultiplayerController.BP_OnlineMultiplayerController_C|SetPlayerIndex _output_get (Utilities|Select :Index (Variables|Default|GetClientIndex) :Option%200 0 :Option%201 1 :Option%202 2 :Option%203 3))
      (Class|BPIMultiplayer|AllocatePlayer(Message) _output_get)
      (bind _asbp_beamerman_multi_player (Utilities|Casting|CastToBP_BeamermanMultiPlayer (Pawn|GetControlledPawn (Variables|Default|GetCurrentPlayer))))
      (Utilities|Array|Add (Variables|Default|GetOnline%20Multi%20Player%20Objects) _asbp_beamerman_multi_player)
      (CallFunction|SetGameState)
      (Utilities|Set|Add (Variables|Default|GetAlivePlayers) _clientindex)
      (Math|Integer|IncrementInt _clientindex))))

(fn ConstructionScript)

(fn SetPlayerCollisions
  (for (_array_element _array_index) (Variables|Default|GetOnline%20Multi%20Player%20Objects)
    (switch int _array_index
      (:0
        (Collision|SetCollisionObjectType (Variables|/Script/Engine.Character|GetCapsuleComponent _array_element) "ECC_GameTraceChannel1"))
      (:1
        (Collision|SetCollisionObjectType (Variables|/Script/Engine.Character|GetCapsuleComponent _array_element) "ECC_GameTraceChannel2"))
      (:2
        (Collision|SetCollisionObjectType (Variables|/Script/Engine.Character|GetCapsuleComponent _array_element) "ECC_GameTraceChannel3"))
      (:3
        (Collision|SetCollisionObjectType (Variables|/Script/Engine.Character|GetCapsuleComponent _array_element) "ECC_GameTraceChannel4"))))
  (bind _aspersistent_game_instance (Utilities|Casting|CastToPersistentGameInstance (Game|GetGameInstance)))
  (for (_array_element_2 _array_index_2) (Variables|Default|GetOnline%20Multi%20Player%20Objects)
    (switch int _array_index_2
      (:0
        (Utilities|Map|Add (Variables|/Game/PersistentGameInstance.PersistentGameInstance_C|GetOnlinePlayerCollisionMappings _aspersistent_game_instance) _array_element_2 (Utilities|Enum|LiteralenumECollisionChannel "ECC_GameTraceChannel1")))
      (:1
        (Utilities|Map|Add (Variables|/Game/PersistentGameInstance.PersistentGameInstance_C|GetOnlinePlayerCollisionMappings _aspersistent_game_instance) _array_element_2 (Utilities|Enum|LiteralenumECollisionChannel "ECC_GameTraceChannel2")))
      (:2
        (Utilities|Map|Add (Variables|/Game/PersistentGameInstance.PersistentGameInstance_C|GetOnlinePlayerCollisionMappings _aspersistent_game_instance) _array_element_2 (Utilities|Enum|LiteralenumECollisionChannel "ECC_GameTraceChannel3")))
      (:3
        (Utilities|Map|Add (Variables|/Game/PersistentGameInstance.PersistentGameInstance_C|GetOnlinePlayerCollisionMappings _aspersistent_game_instance) _array_element_2 (Utilities|Enum|LiteralenumECollisionChannel "ECC_GameTraceChannel4"))))))

(fn RegisterPlayerDeathinGameState
  (params (DeadPlayer :type BP%20Beamerman%20Multi%20Player%20Object%20Reference))
  (bind _output_get (Variables|Default|SetDeadPlayerRef DeadPlayer))
  (Utilities|Array|AddUnique (Variables|/Game/Blueprints/Online_Multiplayer/BP_MultiplayerGameState.BP_MultiplayerGameState_C|GetPlayer%20Death%20Records (Variables|Default|GetMyGameState)) (Utilities|Struct|MakeStruct_PlayerDeath (Variables|/Game/Blueprints/Player/BP_BeamermanMultiPlayer.BP_BeamermanMultiPlayer_C|GetPlayerID _output_get) (- 6e+01 (Variables|/Game/PersistentGameInstance.PersistentGameInstance_C|GetCurrentTimeRemaining (Variables|Default|GetPersistentGameInstanceRef))) (Variables|/Game/Blueprints/Score/OnlineMultiplayerScoreTracker.OnlineMultiplayerScoreTracker_C|GetTotalScore (Variables|/Game/Blueprints/Player/BP_BeamermanMultiPlayer.BP_BeamermanMultiPlayer_C|GetScore%20Tracker _output_get))))
  (Utilities|Set|Remove (Variables|Default|GetAlivePlayers) (Variables|/Game/Blueprints/Player/BP_BeamermanMultiPlayer.BP_BeamermanMultiPlayer_C|GetPlayerID (Variables|Default|GetDeadPlayerRef))))

(fn RegisterPlayerDeathinGameMode
  (params (PlayerRef :type BP%20Beamerman%20Multi%20Player%20Object%20Reference))
  (Utilities|Array|AddUnique (Variables|Default|GetPlayerRecords) (Utilities|Struct|MakeStruct_PlayerDeath (Variables|/Game/Blueprints/Player/BP_BeamermanMultiPlayer.BP_BeamermanMultiPlayer_C|GetPlayerID PlayerRef) (- 6e+01 (Variables|/Game/PersistentGameInstance.PersistentGameInstance_C|GetCurrentTimeRemaining (Variables|Default|GetPersistentGameInstanceRef))) (Variables|/Game/Blueprints/Score/OnlineMultiplayerScoreTracker.OnlineMultiplayerScoreTracker_C|GetTotalScore (Variables|/Game/Blueprints/Player/BP_BeamermanMultiPlayer.BP_BeamermanMultiPlayer_C|GetScore%20Tracker PlayerRef))))
  (return))