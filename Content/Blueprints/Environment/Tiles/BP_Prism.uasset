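; BP_Prism is an environment tile that splits an incoming laser into new beams along its north, south, east and west spawn points.
; On LazerInteract, it spawns a child laser from each point, skipping the one facing back along the incoming beam, and increments that laser's ReflectIndex per child.
; It then sends the laser a destroy message and spawns a shockwave particle at the prism.
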(event EventLazerInteract
  (params (Lazer :type BP%20Laser%20Pulse%20Object%20Reference))
  (for _array_element (Utilities|Array|MakeArray (Variables|Default|GetLazerSpawnNorth) (Variables|Default|GetLazerSpawnSouth) (Variables|Default|GetLazerSpawnEast) (Variables|Default|GetLazerSpawnWest))
    (if (not (Math|Vector|Equal(Vector) (Math|Vector|Normalize (* (Variables|/Game/Blueprints/Projectiles/BP_laserPulse.BP_LaserPulse_C|Getdirection Lazer) -1)) (Math|Vector|GetForwardVector _array_element) 0.0001))
      (Default|SpawnChild Lazer (Math|Vector|GetForwardVector _array_element) (Transformation|GetWorldLocation _array_element) self)
      (Math|Integer|IncrementInt (Variables|/Game/Blueprints/Projectiles/BP_laserPulse.BP_LaserPulse_C|GetReflectIndex Lazer))))
  (Class|BPIInteractable|LazerDestroy(Message) Lazer self)
  (CallFunction|PrismEffects))

(fn ConstructionScript
  (|CallParentFunction))

(fn PrismEffects
  (Effects|SpawnEmitteratLocation "/Game/StarterContent/Particles/P_ShockWave.P_ShockWave" (Transformation|GetWorldLocation (Variables|Default|GetPrism)) "0, 0, 0" "2.000000,2.000000,2.000000"))

(fn LazerSpawn
  (return))