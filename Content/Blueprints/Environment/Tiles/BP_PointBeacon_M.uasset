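; BP_PointBeacon_M is a multiplayer environment beacon that keeps one point orb spawned just above itself.
; A looping timer polls while the game state's CurrentTime is under 60 and checks whether the current orb is still valid.
; When the orb is missing, it pauses the timer, waits a random cooldown, then resumes polling and spawns a replacement.
; The orb reference has an empty OnRep handler.
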(event Custom|SpawnOrb
  (bind _asbp_multiplayer_game_state (Utilities|Casting|CastToBP_MultiplayerGameState (Game|GetGameState)))
  (if (< (Variables|/Game/Blueprints/Player/BP_MultiplayerGameState.BP_MultiplayerGameState_C|GetCurrentTime _asbp_multiplayer_game_state) 60)
    (if (not (Utilities|IsValid (Variables|Default|GetPointOrb)))
      (Utilities|Time|PauseTimerbyHandle (Variables|Default|GetTimer))
      (Utilities|FlowControl|Delay (Math|Random|RandomFloatinRange (Variables|Default|GetMinCooldown) (Variables|Default|GetMaxCooldown)))
      (Utilities|Time|UnpauseTimerbyHandle (Variables|Default|GetTimer))
      (CallFunction|SpawnPointOrb))))

(event Custom|Spawn%20Point%20Orb
  (bind _returnvalue (Game|SpawnActorfromClass "/Game/Blueprints/Environment/BP_PointOrb_M.BP_PointOrb_M_C" (Math|Transform|MakeTransform (+ (Transformation|GetActorLocation) "0,0.000000,50.000000") "0, 0, 0" "1,1,1") "Undefined" 0 0))
  (Variables|Default|SetPointOrb _returnvalue))

(event EventBeginPlay
  (bind _returnvalue (Utilities|Time|SetTimerbyEvent (delegate Custom|SpawnOrb) 0.1 true))
  (Variables|Default|SetTimer _returnvalue))

(fn ConstructionScript
  (|CallParentFunction))

(fn OnRepPointOrb)