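; Diagonal mirror tile that redirects lasers striking it.
; On laser interaction, it sends the laser a destroy message, then has it spawn a child beam at the tile's LaserSpawnPoint with itself as spawner.
; The child's direction reflects the incoming direction about a normal taken from the X vector of the Mirror component's negated world rotation.
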(event EventLazerInteract
  (params (Lazer :type BP%20Laser%20Pulse%20Object%20Reference))
  (Class|BPIInteractable|LazerDestroy(Message) Lazer self)
  (CallFunction|ReconstructLaser Lazer))

(fn ConstructionScript
  (|CallParentFunction))

(fn ReconstructLaser
  (params (laser :type BP%20Laser%20Pulse%20Object%20Reference))
  (Default|SpawnChild laser (Math|Vector|GetReflectionVector (Variables|/Game/Blueprints/Projectiles/BP_laserPulse.BP_LaserPulse_C|Getdirection laser) (Math|Rotator|GetRotationXVector (* (Transformation|GetWorldRotation (Variables|Default|GetMirror)) -1.0))) (Transformation|GetWorldLocation (Variables|Default|GetLaser%20spawn%20point)) self))