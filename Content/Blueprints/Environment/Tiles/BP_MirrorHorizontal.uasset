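; Horizontal mirror tile that redirects lasers hitting it.
; On LazerInteract it asks the incoming laser to spawn a child at that laser's location, with the direction turned by a fixed 180-degree single-axis rotation and the mirror as owner.
; It then sends LazerDestroyMessage to the incoming laser, so redirection works by replacing the beam rather than steering it.
; LazerSpawn is empty and the construction script only calls its parent.
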(event EventLazerInteract
  (params (Lazer :type BP%20Laser%20Pulse%20M%20Object%20Reference))
  (Default|SpawnChild Lazer (Math|Vector|RotateVector (Variables|/Game/Blueprints/Projectiles/BP_LaserPulse_M.BP_LaserPulse_M_C|Getdirection Lazer) "0,180.000000, 0") (Transformation|GetActorLocation Lazer) self)
  (Class|BPIInteractableM|LazerDestroy(Message) Lazer self))

(fn ConstructionScript
  (|CallParentFunction))

(fn LazerSpawn
  (return))