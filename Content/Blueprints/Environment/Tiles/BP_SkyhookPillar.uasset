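; BP_SkyhookPillar is an environment tile pillar that degrades under laser hits and finally explodes.
; LazerInteract notifies the laser, then decrements Stage, swapping damage materials and revealing smoke and a warning indicator when Stage reaches zero.
; A further hit sets the Exploded guard, calls Explode for particles, sound and mesh removal, hides the warning effects and spawns BP_PillarFalling in its place.
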(event EventLazerInteract
  (params (Lazer :type BP%20Laser%20Pulse%20Object%20Reference))
  (if (not (Variables|Default|GetExploded))
    (Class|BPIInteractable|LazerDestroy(Message) Lazer self)
    (if (== (Variables|Default|GetStage) 0)
      (Variables|Default|SetExploded true)
      (CallFunction|Explode)
      (Rendering|SetVisibility (Variables|Default|GetGroundSmoke_PS) false false)
      (Rendering|SetVisibility (Variables|Default|GetSmoking_PS) false false)
      (Rendering|SetVisibility (Variables|Default|GetWarningIndicator) false false)
      (Game|SpawnActorfromClass "/Game/Blueprints/Environment/BP_PillarFalling.BP_PillarFalling_C" (Math|Transform|MakeTransform (Transformation|GetActorLocation) "0, 0, 0" "1,1,1") "Undefined" 0 0)
      (else
        ;[1 1 1] If one hit left on Pillar
        (bind _output_get (Variables|Default|SetStage (- (Variables|Default|GetStage) 1)))
        (if (== _output_get 1)
          (Rendering|Material|SetMaterial (Variables|Default|GetPillar) 0 "/Game/Materials/Props/Barrels/MI_Barrel_Red_Stage2.MI_Barrel_Red_Stage2")
          (else
            ;[1 1 1] If zero hit left on Pillar
            (if (== _output_get 0)
              (Rendering|SetVisibility (Variables|Default|GetGroundSmoke_PS) true false)
              (Rendering|SetVisibility (Variables|Default|GetSmoking_PS) true false)
              (Rendering|Material|SetMaterial (Variables|Default|GetPillar) 0 "/Game/Materials/Props/Barrels/MI_Barrel_Red_Stage3.MI_Barrel_Red_Stage3")
              (Rendering|SetVisibility (Variables|Default|GetWarningIndicator) true false))))))))

(fn ConstructionScript
  (|CallParentFunction))

(fn Explode
  (bind _returnvalue (Transformation|GetActorLocation))
  (bind _returnvalue_2 (+ _returnvalue "0, 0,50.000000"))
  (Effects|SpawnEmitteratLocation "/Game/StarterContent/Particles/P_Explosion.P_Explosion" _returnvalue_2)
  (Audio|SpawnSoundatLocation "/Game/Audio/SFX/SW_Explosion_1.SW_Explosion_1" _returnvalue_2 "0, 0, 0" 1.0 1.0 0.0 0 0)
  (Components|DestroyComponent (Variables|Default|GetPillar)))

(fn LazerSpawn
  (return))