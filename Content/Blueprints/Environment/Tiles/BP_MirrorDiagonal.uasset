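; BP_MirrorDiagonal is a mirror tile that reflects laser pulses when it receives LazerInteract.
; While bounces remain, ReconstructLaser replaces the pulse with a new BP_LaserPulse at the mirror, reflecting its direction, decrementing ReflectIndex, restoring range and keeping its Spawner.
; With none left, it calls LazerDestroy on the pulse; both outcomes emit sparks.
; AlterLaser, an in-place redirect alternative, is never run.
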(event EventBeginPlay
  (|CallParentFunction) ; This node is disabled and will not be called.\nDrag off pins to build functionality.
)

(event EventLazerInteract
  (params (Lazer :type BP%20Laser%20Pulse%20Object%20Reference))
  (if (> (Variables|/Game/Blueprints/Projectiles/BP_laserPulse.BP_LaserPulse_C|GetReflectIndex Lazer) 0)
    (CallFunction|ReconstructLaser Lazer)
    (else
      (Effects|SpawnEmitteratLocation "/Game/StarterContent/Particles/P_bounceSpark.P_bounceSpark" (Transformation|GetWorldLocation (Variables|Default|GetMirror)))
      (Default|LazerDestroy Lazer))))

(event EventTick
  (params (DeltaSeconds :type Float%20%28single-precision%29))
  (|CallParentFunction DeltaSeconds) ; This node is disabled and will not be called.\nDrag off pins to build functionality.
)

(fn ConstructionScript
  (|CallParentFunction))

(fn AlterLaser
  (params (Laser :type BP%20Laser%20Pulse%20Object%20Reference))
  (bind _mirror (Variables|Default|GetMirror))
  (bind _returnvalue (Transformation|GetWorldLocation _mirror))
  (Variables|/Game/Blueprints/Projectiles/BP_laserPulse.BP_LaserPulse_C|Setdirection Laser (Math|Vector|GetReflectionVector (Variables|/Game/Blueprints/Projectiles/BP_laserPulse.BP_LaserPulse_C|Getdirection Laser) (Math|Rotator|GetRotationXVector (* (Transformation|GetWorldRotation (Variables|Default|GetMirror)) -1.0))))
  (bind _result (Math|Integer|DecrementInt (Variables|/Game/Blueprints/Projectiles/BP_laserPulse.BP_LaserPulse_C|GetReflectIndex Laser))
    (:%20%20
      (Variables|/Game/Blueprints/Projectiles/BP_laserPulse.BP_LaserPulse_C|SetReflectIndex Laser _result)
      (Variables|/Game/Blueprints/Projectiles/BP_laserPulse.BP_LaserPulse_C|SetRange Laser (Variables|/Game/Blueprints/Projectiles/BP_laserPulse.BP_LaserPulse_C|GetOriginalRange Laser))
      (Transformation|SetActorLocation Laser _returnvalue false false)
      (Effects|SpawnEmitteratLocation "/Game/StarterContent/Particles/P_bounceSpark.P_bounceSpark" _returnvalue "0, 0, 0" "2.000000,2.000000,2.000000"))))

(fn ReconstructLaser
  (params (laser :type BP%20Laser%20Pulse%20Object%20Reference))
  (bind _mirror (Variables|Default|GetMirror))
  (LocalVariables|SetSpawner (Variables|/Game/Blueprints/Projectiles/BP_laserPulse.BP_LaserPulse_C|GetSpawner laser))
  (bind _output_get (LocalVariables|Settemp%20ref%20index (Variables|/Game/Blueprints/Projectiles/BP_laserPulse.BP_LaserPulse_C|GetReflectIndex laser)))
  (Math|Integer|DecrementInt _output_get
    (:%20%20
      (LocalVariables|SetTemp%20direction (Math|Vector|GetReflectionVector (Variables|/Game/Blueprints/Projectiles/BP_laserPulse.BP_LaserPulse_C|Getdirection laser) (Math|Rotator|GetRotationXVector (* (Transformation|GetWorldRotation (Variables|Default|GetMirror)) -1.0))))
      (LocalVariables|SettempRange (Variables|/Game/Blueprints/Projectiles/BP_laserPulse.BP_LaserPulse_C|GetOriginalRange laser))
      (Effects|SpawnEmitteratLocation "/Game/StarterContent/Particles/P_bounceSpark.P_bounceSpark" (Transformation|GetWorldLocation _mirror) "0, 0, 0" "2.000000,2.000000,2.000000")
      (bind _returnvalue (Game|SpawnActorfromClass "/Game/Blueprints/Projectiles/BP_laserPulse.BP_LaserPulse_C" (Transformation|GetWorldTransform _mirror) "Undefined" 0 0))
      (Variables|/Game/Blueprints/Projectiles/BP_laserPulse.BP_LaserPulse_C|Setdirection _returnvalue (LocalVariables|GetTemp%20direction))
      (Variables|/Game/Blueprints/Projectiles/BP_laserPulse.BP_LaserPulse_C|SetReflectIndex _returnvalue (LocalVariables|Gettemp%20ref%20index))
      (Variables|/Game/Blueprints/Projectiles/BP_laserPulse.BP_LaserPulse_C|SetRange _returnvalue (LocalVariables|GettempRange))
      (Variables|/Game/Blueprints/Projectiles/BP_laserPulse.BP_LaserPulse_C|SetSpawner _returnvalue (LocalVariables|GetSpawner))
      (Actor|DestroyActor laser))))