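; BP_SkyPillar is a destructible environment pillar that lasers wear down stage by stage until it explodes.
; Each laser hit triggers the laser's destroy message and dust, then decrements Stage or, at zero, explodes the pillar.
; The explosion removes the crate with effects, makes overlapping BP_BaseTiles fall and registers them in the game's fall array.
; It also defines random powerup spawning, uncalled here, and an empty LazerSpawn.
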(event EventLazerInteract
  (params (Lazer :type BP%20Laser%20Pulse%20Object%20Reference))
  (if (not (Variables|Default|GetExploded))
    (Class|BPIInteractable|LazerDestroy(Message) Lazer self)
    (Effects|SpawnEmitteratLocation "/Game/StarterContent/Particles/P_Ambient_Dust.P_Ambient_Dust" "0, 0, 0")
    (if (== 0 (Variables|Default|GetStage))
      (Variables|Default|SetExploded true)
      (CallFunction|Explode)
      (for _array_element (Collision|GetOverlappingActors (Variables|Default|GetBoxCollsion) 0 :!class /Script/Engine.PrimitiveComponent)
        (bind _asbp_base_tile (Utilities|Casting|CastToBP_BaseTile _array_element))
        (Default|TileFallAction _asbp_base_tile)
        (Default|AddtoGameTileFallArray _asbp_base_tile))
      (else
        (Variables|Default|SetStage (- (Variables|Default|GetStage) 1))))))

(fn ConstructionScript
  (|CallParentFunction))

(fn Explode
  (bind _returnvalue (Transformation|GetActorLocation))
  (bind _returnvalue_2 (+ _returnvalue "0, 0,50.000000"))
  (Effects|SpawnEmitteratLocation "/Game/StarterContent/Particles/P_Explosion.P_Explosion" _returnvalue_2)
  (Audio|SpawnSoundatLocation "/Game/Audio/SFX/SW_Explosion_1.SW_Explosion_1" _returnvalue_2 "0, 0, 0" 1.0 1.0 0.0 0 0)
  (Components|DestroyComponent (Variables|Default|GetCrate)))

(fn SpawnPowerup
  (bind _powerupclass (CallFunction|ChoosePowerup))
  (Game|SpawnActorfromClass _powerupclass (Math|Transform|MakeTransform (Transformation|GetWorldLocation (Variables|Default|GetBox)) "0, 0, 0" "1,1,1") "Undefined" 0 0))

(fn ChoosePowerup
  (bind _possiblepowerupsarray (Variables|Default|GetPossiblePowerUpsArray))
  (return (Utilities|Array|Get(acopy) _possiblepowerupsarray (Math|Random|RandomInteger (Utilities|Array|Length _possiblepowerupsarray)))))

(fn LazerSpawn
  (return))