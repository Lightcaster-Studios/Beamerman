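; Diagonal mirror tile that reflects lasers and lets AI bots trace shots off its surface.
; On laser contact it spawns a child laser from the mirror along the reflected direction, then sends the incoming laser a destroy message.
; AI traces use the same reflection over the bot's fire range, with persistent debug drawing.
; Any hit is sent back to the controller with this mirror as reflector.
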(event EventLazerInteract
  (params (Lazer :type BP%20Laser%20Pulse%20M%20Object%20Reference))
  (CallFunction|ReconstructLaser Lazer)
  (Class|BPIInteractableM|LazerDestroy(Message) Lazer self))

(event EventTracefromIncidence
  (params (Direction :type Vector :default "0, 0, 0") (SpawnController :type AI%20Controller%20Object%20Reference))
  (bind (_hit _hit_actor _reflector) (CallFunction|Retrace Direction SpawnController))
  (if _hit
    (Class|BPITraceable|ReverseTrace(Message) SpawnController _hit_actor _reflector)))

(fn ConstructionScript
  (|CallParentFunction))

(fn ReconstructLaser
  (params (laser :type BP%20Laser%20Pulse%20M%20Object%20Reference))
  (Default|SpawnChild laser (Math|Vector|GetReflectionVector (Variables|/Game/Blueprints/Projectiles/BP_LaserPulse_M.BP_LaserPulse_M_C|Getdirection laser) (Math|Rotator|GetRotationXVector (* (Transformation|GetWorldRotation (Variables|Default|GetMirror)) -1.0))) (Transformation|GetWorldLocation (Variables|Default|GetMirror)) self))

(fn Retrace
  (params (Direction :type Vector) (Controller :type AI%20Controller%20Object%20Reference))
  (bind _mirror (Variables|Default|GetMirror))
  (bind _returnvalue (Transformation|GetWorldLocation _mirror))
  (bind _asai_bot_controller (Utilities|Casting|CastToAI_botController Controller))
  (bind (_outhit _returnvalue_2) (Collision|LineTraceByChannel _returnvalue (+ (* (Math|Vector|GetReflectionVector Direction (Math|Rotator|GetRotationXVector (* (Transformation|GetWorldRotation (Variables|Default|GetMirror)) -1.0))) (Variables|/Game/Blueprints/AIPlayer/AI_botController.AI_botController_C|GetFire%20Trace%20Range _asai_bot_controller)) _returnvalue) "TraceTypeQuery1" false 0 "Persistent"))
  (return _returnvalue_2 (.HitActor (Collision|BreakHitResult _outhit)) self))