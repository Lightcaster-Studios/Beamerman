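; BP_MirrorWalledDiagonal_M is a diagonal walled mirror tile that redirects lasers hitting it.
; On LazerInteract it spawns a child laser at LaserSpawnPoint, owned by the tile, then sends the incoming laser a destroy message.
; The child's direction reflects the incoming direction about a normal taken from the X vector of MirrorMiddle's negated world rotation.
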(event EventLazerInteract
  (params (Lazer :type BP%20Laser%20Pulse%20M%20Object%20Reference))
  (CallFunction|ReconstructLaser Lazer)
  (Class|BPIInteractableM|LazerDestroy(Message) Lazer self))

(fn ConstructionScript
  (|CallParentFunction))

(fn ReconstructLaser
  (params (laser :type BP%20Laser%20Pulse%20M%20Object%20Reference))
  (Default|SpawnChild laser (Math|Vector|GetReflectionVector (Variables|/Game/Blueprints/Projectiles/BP_LaserPulse_M.BP_LaserPulse_M_C|Getdirection laser) (Math|Rotator|GetRotationXVector (* (Transformation|GetWorldRotation (Variables|Default|GetMirrorMiddle)) -1.0))) (Transformation|GetWorldLocation (Variables|Default|GetLaserSpawnPoint)) self))