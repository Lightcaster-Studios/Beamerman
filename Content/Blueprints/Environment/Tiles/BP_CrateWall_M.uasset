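; BP_CrateWall_M is a destructible crate wall tile that explodes when hit by a lazer and may drop a random powerup.
; Two near-identical lazer events notify the lazer, set a one-shot Exploded flag, and play explosion effects and sound through duplicate Explode and Explosion routines.
; Only the Crate component is destroyed.
; A percentage roll then decides whether a class from PossiblePowerUpsArray spawns at the Box location.
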(event Custom|L_Interact
  (params (Lazer :type BP%20Laser%20Pulse%20M%20Object%20Reference))
  (if (not (Variables|Default|GetExploded))
    (Class|BPIInteractableM|LazerDestroy(Message) Lazer self)
    (Variables|Default|SetExploded true)
    (CallFunction|Explode)
    (if (<= (Math|Random|RandomIntegerinRange 1 100) (Variables|Default|GetPowerUpSpawnChance))
      (CallFunction|SpawnPowerup))))

(event Custom|Explosion
  (bind _returnvalue (Transformation|GetActorLocation))
  (bind _returnvalue_2 (+ _returnvalue "0, 0,50.000000"))
  (Effects|SpawnEmitteratLocation "/Game/StarterContent/Particles/P_Explosion.P_Explosion" _returnvalue_2)
  (Audio|SpawnSoundatLocation "/Game/Audio/SFX/SW_Explosion_1.SW_Explosion_1" _returnvalue_2 "0, 0, 0" 1.0 1.0 0.0 0 0)
  (Components|DestroyComponent (Variables|Default|GetCrate)))

(event EventLazerInteract
  (params (Lazer :type BP%20Laser%20Pulse%20M%20Object%20Reference))
  (if (not (Variables|Default|GetExploded))
    (Class|BPIInteractableM|LazerDestroy(Message) Lazer self)
    (Variables|Default|SetExploded true)
    (CallFunction|Explosion)
    (if (<= (Math|Random|RandomIntegerinRange 1 100) (Variables|Default|GetPowerUpSpawnChance))
      (CallFunction|SpawnPowerup))))

(fn ConstructionScript
  (|CallParentFunction))

(fn Explode
  (bind _returnvalue (Transformation|GetActorLocation))
  (bind _returnvalue_2 (+ _returnvalue "0, 0,50.000000"))
  (Effects|SpawnEmitteratLocation "/Game/StarterContent/Particles/P_Explosion.P_Explosion" _returnvalue_2)
  (Audio|SpawnSoundatLocation "/Game/Audio/SFX/SW_Explosion_1.SW_Explosion_1" _returnvalue_2 "0, 0, 0" 1.0 1.0 0.0 0 0)
  (Components|DestroyComponent (Variables|Default|GetCrate)))

(fn SpawnPowerup
  (bind _powerupclass (CallFunction|ChoosePowerup))
  (Game|SpawnActorfromClass _powerupclass (Math|Transform|MakeTransform (Transformation|GetWorldLocation (Variables|Default|GetBox)) "0, 0, 0" "1,1,1") "Undefined" 0 0))

(fn ChoosePowerup
  (bind _possiblepowerupsarray (Variables|Default|GetPossiblePowerUpsArray))
  (return (Utilities|Array|Get(acopy) _possiblepowerupsarray (Math|Random|RandomInteger (Utilities|Array|Length _possiblepowerupsarray)))))

(fn LazerSpawn
  (return))