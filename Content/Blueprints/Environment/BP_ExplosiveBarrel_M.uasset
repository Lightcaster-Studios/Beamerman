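; Explosive barrel actor that sits on a grid tile, optionally dropping in first, and explodes when hit by a laser.
; A looping timer steps it down until Height runs out, then OnGround flags the overlapped BP_BaseTile as occupied and disables physics simulation.
; LazerInteract fires once, notifying the laser and spawning BP_BarrelExplosion_M before freeing the tile and destroying the barrel with particles and sound.
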(event Custom|On%20Ground
  (for _array_element (Collision|GetOverlappingActors (Variables|Default|GetBarrel) "/Game/Blueprints/Environment/BP_BaseTile.BP_BaseTile_C" :!class /Script/Engine.PrimitiveComponent)
    (bind _asbp_base_tile (Utilities|Casting|CastToBP_BaseTile _array_element))
    (bind _output_get (Variables|Default|SetBaseTile _asbp_base_tile))
    (Variables|/Game/Blueprints/Environment/BP_BaseTile.BP_BaseTile_C|SetHasBarrel _output_get true)
    (Utilities|FlowControl|Delay 0.2)
    (Physics|SetSimulatePhysics (Variables|Default|GetBarrel) false)))

(event Custom|Spawn%20Explosion
  (Game|SpawnActorfromClass "/Game/Blueprints/Environment/BP_BarrelExplosion_M.BP_BarrelExplosion_M_C" (Math|Transform|MakeTransform (Transformation|GetActorLocation) "0, 0, 0" "1,1,1") "Undefined" 0 0)
  (Variables|/Game/Blueprints/Environment/BP_BaseTile.BP_BaseTile_C|SetHasBarrel (Variables|Default|GetBaseTile) false)
  (CallFunction|Explode))

(event EventBeginPlay
  (Utilities|FlowControl|Delay (Variables|Default|GetInterval))
  (if (Variables|Default|GetDropping)
    (bind _returnvalue (Utilities|Time|SetTimerbyFunctionName self "Falling" (Variables|Default|GetInterval) true))
    (Variables|Default|SetTimer _returnvalue)
    (else
      (CallFunction|OnGround))))

(event EventLazerInteract
  (params (Lazer :type BP%20Laser%20Pulse%20M%20Object%20Reference))
  (if (not (Variables|Default|GetExploded))
    (Variables|Default|SetExploded true)
    (Class|BPIInteractableM|LazerDestroy(Message) Lazer self)
    (CallFunction|SpawnExplosion)))

(fn ConstructionScript)

(fn Explode
  (bind _returnvalue (Transformation|GetActorLocation))
  (bind _returnvalue_2 (+ _returnvalue "0, 0,50.000000"))
  (Effects|SpawnEmitteratLocation "/Game/StarterContent/Particles/P_Explosion.P_Explosion" _returnvalue_2)
  (Audio|SpawnSoundatLocation "/Game/Audio/SFX/SW_Explosion_1.SW_Explosion_1" _returnvalue_2 "0, 0, 0" 1.0 1.0 0.0 0 0)
  (Actor|DestroyActor))

(fn Falling
  (if (> (Variables|Default|GetHeight) 0.0)
    (Transformation|AddActorWorldOffset (Math|Vector|MakeVector 0.0 0.0 (Variables|Default|GetFallSpeed)))
    (if (<= (+ (Variables|Default|GetHeight) (Variables|Default|GetFallSpeed)) 0.0)
      (Variables|Default|SetHeight 0.0)
      (else
        (Variables|Default|SetHeight (+ (Variables|Default|GetHeight) (Variables|Default|GetFallSpeed)))))
    (else
      (Utilities|Time|ClearandInvalidateTimerbyHandle (Variables|Default|GetTimer))
      (CallFunction|OnGround))))