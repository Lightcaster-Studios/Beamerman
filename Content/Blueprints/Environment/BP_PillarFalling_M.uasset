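; BP_PillarFalling_M is a one-shot area trigger that makes the floor tiles within its box fall, apparently as the effect of a falling pillar.
; On BeginPlay it resizes its box collision to the Size variable, then gathers the overlapping BP_BaseTile actors.
; It calls TileFallAction on each tile, then destroys itself immediately, with no tick or timer.
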(event Custom|Pillar%20falling
  (Components|Box|SetBoxExtent (Variables|Default|GetBoxCollision) (Variables|Default|GetSize) true)
  (for _array_element (Collision|GetOverlappingActors (Variables|Default|GetBoxCollision) "/Game/Blueprints/Environment/BP_BaseTile.BP_BaseTile_C" :!class /Script/Engine.PrimitiveComponent)
    (bind _asbp_base_tile (Utilities|Casting|CastToBP_BaseTile _array_element))
    (Default|TileFallAction _asbp_base_tile))
  (Actor|DestroyActor))

(event EventBeginPlay
  (CallFunction|PillarFalling))

(fn ConstructionScript)