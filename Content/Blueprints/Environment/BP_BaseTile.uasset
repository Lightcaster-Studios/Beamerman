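; Base environment tile that becomes a candidate to fall as neighboring tiles leave it.
; FindNumNeighbors counts adjacent tiles through box overlap testers under TileOverlapTesters.
; When another tile ends overlap, the count drops, and below four the tile registers once in PersistentGameInstance's TileFallCandidates.
; TileFallAction performs the fall by enabling physics on the root; neither it nor the neighbor count is called within this Blueprint.
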(event Custom|TryTriggerTileFall
  (params (Triggering%20Actor :type Actor%20Object%20Reference))
  (bind _isvalid (CallFunction|CheckTileFallValidity Triggering%20Actor))
  (if _isvalid
    (CallFunction|AddtoGameTileFallArray)))

(event Collision|EventActorEndOverlap
  (params (OtherActor :type Actor%20Object%20Reference))
  (CallFunction|TryTriggerTileFall OtherActor))

(fn ConstructionScript)

(fn TileFallAction
  (Physics|SetSimulatePhysics (Variables|Default|GetSceneRoot) true))

(fn FindNumNeighbors
  (for _array_element (Components|GetChildrenComponents (Variables|Default|GetTileOverlapTesters) false)
    (bind _asbox_collision (Utilities|Casting|CastToBoxComponent _array_element))
    (bind _returnvalue (Collision|ComponentOverlapActors _asbox_collision (Transformation|GetWorldTransform _asbox_collision) (Utilities|Array|MakeArray "ObjectTypeQuery2") "BP_BaseTile_C"))
    (if _returnvalue
      (Math|Integer|IncrementInt (Variables|Default|GetNumNeighbors))))
  (return (Variables|Default|GetNumNeighbors)))

(fn AddtoGameTileFallArray
  (bind _aspersistent_game_instance (Utilities|Casting|CastToPersistentGameInstance (Game|GetGameInstance)))
  (Utilities|Array|AddUnique (Variables|/Game/PersistentGameInstance.PersistentGameInstance_C|GetTileFallCandidates _aspersistent_game_instance) self)
  (Variables|Default|SetIsScheduledToFall true))

(fn CheckTileFallValidity
  (params (Leaving%20Actor :type Actor%20Object%20Reference))
  (if (not (Variables|Default|GetIsScheduledToFall))
    (Utilities|Casting|CastToBP_BaseTile Leaving%20Actor
      (:then
        (bind _result (Math|Integer|DecrementInt (Variables|Default|GetNumNeighbors))
          (:%20%20
            (return (and (< _result 4) true)))))
      (:CastFailed
        _)))
  (return false))