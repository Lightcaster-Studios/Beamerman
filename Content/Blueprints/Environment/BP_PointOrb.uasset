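; BP_PointOrb is a point orb pickup that players collect by overlapping its box.
; The overlap casts to the Beamerman player or multiplayer player, reports the pickup with player and orb, then calls TriggerPowerup.
; It builds on a parent class, passing BeginPlay and construction through, while its PowerUpEffect only plays a pickup sound at the orb's location.
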(event OnComponentBeginOverlap(Box)
  (params (OverlappedComponent :type Primitive%20Component%20Object%20Reference) (OtherActor :type Actor%20Object%20Reference) (OtherComp :type Primitive%20Component%20Object%20Reference) (OtherBodyIndex :type Integer) (bFromSweep :type Boolean) (SweepResult :type Hit%20Result%20Structure%20%28by%20ref%29))
  (bind _asbp_beamerman_player (Utilities|Casting|CastToBP_BeamermanPlayer OtherActor)
    (:then
      (CallFunction|PointOrbReportPickup _asbp_beamerman_player self)
      (CallFunction|TriggerPowerup _asbp_beamerman_player))
    (:CastFailed
      (bind _asbp_beamerman_multi_player (Utilities|Casting|CastToBP_BeamermanMultiPlayer OtherActor))
      (CallFunction|PointOrbReportPickup _asbp_beamerman_multi_player self)
      (CallFunction|TriggerPowerup _asbp_beamerman_multi_player))))

(event EventBeginPlay
  (|CallParentFunction))

(fn ConstructionScript
  (|CallParentFunction))

(fn PowerUpEffect
  (params (Player :type BP%20Beamerman%20Player%20Object%20Reference))
  (Audio|PlaySoundatLocation "/Game/Audio/SFX/PowerUpPickup.PowerUpPickup" (Transformation|GetActorLocation) "0, 0, 0" 1.0 1.0 0.0 0 0 0))