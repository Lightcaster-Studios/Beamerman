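; BP_BarrelExplosion_M is a one-shot explosion area actor that applies the laser interaction to actors caught in its box.
; On BeginPlay it resizes BoxCollision to Size, then sends LazerInteractMessage to each overlapping multiplayer Beamerman, crate wall, skyhook pillar or explosive barrel through per-class casts.
; Hit barrels receive the same message as other targets, and the actor destroys itself immediately after the single overlap pass.
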(event EventBeginPlay
  (Components|Box|SetBoxExtent (Variables|Default|GetBoxCollision) (Variables|Default|GetSize) true)
  (for _array_element (Collision|GetOverlappingActors (Variables|Default|GetBoxCollision) 0 :!class /Script/Engine.PrimitiveComponent)
    (Utilities|FlowControl|Sequence
      (:then_0
        (bind _asbp_beamerman_multi_player (Utilities|Casting|CastToBP_BeamermanMultiPlayer _array_element))
        (Class|BPIInteractableM|LazerInteract(Message) _asbp_beamerman_multi_player))
      (:then_1
        (bind _asbp_crate_wall_m (Utilities|Casting|CastToBP_CrateWall_M _array_element))
        (Class|BPIInteractableM|LazerInteract(Message) _asbp_crate_wall_m))
      (:then_2
        (bind _asbp_skyhook_pillar_m (Utilities|Casting|CastToBP_SkyhookPillar_M _array_element))
        (Class|BPIInteractableM|LazerInteract(Message) _asbp_skyhook_pillar_m))
      (:then_3
        (bind _asbp_explosive_barrel_m (Utilities|Casting|CastToBP_ExplosiveBarrel_M _array_element))
        (Class|BPIInteractableM|LazerInteract(Message) _asbp_explosive_barrel_m))))
  (Actor|DestroyActor))

(fn ConstructionScript)