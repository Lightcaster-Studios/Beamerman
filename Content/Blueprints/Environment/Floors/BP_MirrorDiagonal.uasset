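; Diagonal mirror floor piece that bounces lasers, spawned or moving actors that call its LazerInteract event on contact.
; While the laser has reflections left, it decrements the count, restores range, reflects direction off the mirror's rotation-derived normal and adds an acos-based yaw.
; It then moves the laser to the mirror and spawns a spark.
; With none left, it destroys the laser; LazerSpawn is an empty stub.
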(event EventBeginPlay
  (|CallParentFunction) ; This node is disabled and will not be called.\nDrag off pins to build functionality.
)

(event EventTick
  (params (DeltaSeconds :type Float%20%28single-precision%29))
  (|CallParentFunction DeltaSeconds) ; This node is disabled and will not be called.\nDrag off pins to build functionality.
)

(event EventLazerInteract
  (params (Lazer :type BP%20Laser%20Pulse%20Object%20Reference))
  (bind _mirror (Variables|Default|GetMirror))
  (bind _returnvalue (Transformation|GetWorldLocation _mirror))
  (if (> (Variables|/Game/Blueprints/Projectiles/BP_laserPulse.BP_LaserPulse_C|GetReflectIndex Lazer) 0)
    (Development|PrintString (Utilities|String|ToString(Integer) (Variables|/Game/Blueprints/Projectiles/BP_laserPulse.BP_LaserPulse_C|GetReflectIndex Lazer)))
    (bind _result (Math|Integer|DecrementInt (Variables|/Game/Blueprints/Projectiles/BP_laserPulse.BP_LaserPulse_C|GetReflectIndex Lazer))
      (:%20%20
        (Variables|/Game/Blueprints/Projectiles/BP_laserPulse.BP_LaserPulse_C|SetReflectIndex Lazer _result)
        (Variables|/Game/Blueprints/Projectiles/BP_laserPulse.BP_LaserPulse_C|SetRange Lazer (Variables|/Game/Blueprints/Projectiles/BP_laserPulse.BP_LaserPulse_C|GetOriginalRange Lazer))
        (Variables|/Game/Blueprints/Projectiles/BP_laserPulse.BP_LaserPulse_C|Setdirection Lazer (Math|Vector|GetReflectionVector (Variables|/Game/Blueprints/Projectiles/BP_laserPulse.BP_LaserPulse_C|Getdirection Lazer) (Math|Rotator|GetRotationXVector (* (Transformation|GetWorldRotation (Variables|Default|GetMirror)) -1.0))))
        (Class|Actor|AddActorWorldRotation Lazer (Math|Rotator|MakeRotator 0.0 0.0 (Class|KismetMathLibrary|DegAcos (/ (Math|Vector|DotProduct (Variables|/Game/Blueprints/Projectiles/BP_laserPulse.BP_LaserPulse_C|Getdirection Lazer) (Math|Vector|GetReflectionVector (Variables|/Game/Blueprints/Projectiles/BP_laserPulse.BP_LaserPulse_C|Getdirection Lazer) (Math|Rotator|GetRotationXVector (* (Transformation|GetWorldRotation (Variables|Default|GetMirror)) -1.0)))) (* (Math|Vector|VectorLength (Variables|/Game/Blueprints/Projectiles/BP_laserPulse.BP_LaserPulse_C|Getdirection Lazer)) (Math|Vector|VectorLength (Math|Vector|GetReflectionVector (Variables|/Game/Blueprints/Projectiles/BP_laserPulse.BP_LaserPulse_C|Getdirection Lazer) (Math|Rotator|GetRotationXVector (* (Transformation|GetWorldRotation (Variables|Default|GetMirror)) -1.0)))))))))
        (Transformation|SetActorLocation Lazer _returnvalue false false)
        (Effects|SpawnEmitteratLocation "/Game/StarterContent/Particles/P_bounceSpark.P_bounceSpark" _returnvalue "0, 0, 0" "2.000000,2.000000,2.000000")))
    (else
      (Development|PrintString (Utilities|String|ToString(Integer) (Variables|/Game/Blueprints/Projectiles/BP_laserPulse.BP_LaserPulse_C|GetReflectIndex Lazer)))
      (Default|LazerDestroy Lazer))))

(fn ConstructionScript
  (|CallParentFunction))

(fn LazerSpawn
  (return 0))