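; Horizontal mirror floor Blueprint that bounces lasers back the way they came.
; On LazerInteract, a laser with reflections left uses one up, resets its range, reverses direction, rotates 180 degrees and snaps to the Mirror component with a spark effect.
; A laser with none left is destroyed.
; The same laser actor is reused for each bounce, and the LazerSpawn function is empty.
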(event EventBeginPlay
  (|CallParentFunction) ; This node is disabled and will not be called.\nDrag off pins to build functionality.
)

(event EventTick
  (params (DeltaSeconds :type Float%20%28single-precision%29))
  (|CallParentFunction DeltaSeconds) ; This node is disabled and will not be called.\nDrag off pins to build functionality.
)

(event EventLazerInteract
  (params (Lazer :type BP%20Laser%20Pulse%20Object%20Reference))
  (bind _mirror (Variables|Default|GetMirror))
  (bind _returnvalue (Transformation|GetWorldLocation _mirror))
  (if (> (Variables|/Game/Blueprints/Projectiles/BP_laserPulse.BP_LaserPulse_C|GetReflectIndex Lazer) 0)
    (bind _result (Math|Integer|DecrementInt (Variables|/Game/Blueprints/Projectiles/BP_laserPulse.BP_LaserPulse_C|GetReflectIndex Lazer))
      (:%20%20
        (Variables|/Game/Blueprints/Projectiles/BP_laserPulse.BP_LaserPulse_C|SetReflectIndex Lazer _result)
        (Variables|/Game/Blueprints/Projectiles/BP_laserPulse.BP_LaserPulse_C|SetRange Lazer (Variables|/Game/Blueprints/Projectiles/BP_laserPulse.BP_LaserPulse_C|GetOriginalRange Lazer))
        (Variables|/Game/Blueprints/Projectiles/BP_laserPulse.BP_LaserPulse_C|Setdirection Lazer (* (Variables|/Game/Blueprints/Projectiles/BP_laserPulse.BP_LaserPulse_C|Getdirection Lazer) -1))
        (Class|Actor|AddActorWorldRotation Lazer "0,180.000000, 0")
        (Transformation|SetActorLocation Lazer _returnvalue false false)
        (Effects|SpawnEmitteratLocation "/Game/StarterContent/Particles/P_bounceSpark.P_bounceSpark" _returnvalue "0, 0, 0" "2.000000,2.000000,2.000000")))
    (else
      (Default|LazerDestroy Lazer))))

(fn ConstructionScript
  (|CallParentFunction))

(fn LazerSpawn
  (return 0))