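; A prism actor that splits an incoming laser into four new BP_laserPulsePrism pulses.
; The construction script caches directions, positions and rotations from four Scene marker components around the Cube.
; LazerInteract destroys the laser and, if it has reflections left, plays a spark and calls ShootBeams to spawn a pulse at each marker.
; The range passed to ShootBeams goes unused, SplitBeam is never called here, and LazerSpawn is empty.
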(event EventBeginPlay
  (|CallParentFunction) ; This node is disabled and will not be called.\nDrag off pins to build functionality.
)

(event Collision|EventActorBeginOverlap
  (params (OtherActor :type Actor%20Object%20Reference))
  (|CallParentFunction OtherActor) ; This node is disabled and will not be called.\nDrag off pins to build functionality.
)

(event EventTick
  (params (DeltaSeconds :type Float%20%28single-precision%29))
  (|CallParentFunction DeltaSeconds) ; This node is disabled and will not be called.\nDrag off pins to build functionality.
)

(event EventLazerInteract
  (params (Lazer :type BP%20Laser%20Pulse%20Object%20Reference))
  (Development|PrintString "Hello")
  (if (> (Variables|/Game/Blueprints/Projectiles/BP_laserPulse.BP_LaserPulse_C|GetReflectIndex Lazer) 0)
    (bind _result (Math|Integer|DecrementInt (Variables|/Game/Blueprints/Projectiles/BP_laserPulse.BP_LaserPulse_C|GetReflectIndex Lazer))
      (:%20%20
        (Variables|Default|SetTempRefIndex _result)
        (bind _output_get (Variables|Default|SettempRange (Variables|/Game/Blueprints/Projectiles/BP_laserPulse.BP_LaserPulse_C|GetOriginalRange Lazer)))
        (Default|LazerDestroy Lazer)
        (Effects|SpawnEmitteratLocation "/Game/StarterContent/Particles/P_bounceSpark.P_bounceSpark" (Transformation|GetWorldLocation (Variables|Default|GetCube)) "0, 0, 0" "2.000000,2.000000,2.000000")
        (CallFunction|ShootBeams _output_get)))
    (else
      (Default|LazerDestroy Lazer)
      (Development|PrintString "ref = 0"))))

(fn ConstructionScript
  (bind _scene2 (Variables|Default|GetScene2))
  (bind _scene3 (Variables|Default|GetScene3))
  (bind _cube (Variables|Default|GetCube))
  (bind _scene (Variables|Default|GetScene))
  (bind _scene1 (Variables|Default|GetScene1))
  (bind _returnvalue (Transformation|GetWorldLocation _scene1))
  (bind _returnvalue_2 (Transformation|GetWorldLocation _scene3))
  (bind _returnvalue_3 (Transformation|GetWorldLocation _scene2))
  (bind _returnvalue_4 (Transformation|GetWorldLocation _scene))
  (bind _returnvalue_5 (Transformation|GetWorldLocation _cube))
  (|CallParentFunction)
  (Variables|Default|SetdirArray (Utilities|Array|MakeArray (Math|Vector|GetUnitDirection(Vector) _returnvalue_5 _returnvalue_4) (Math|Vector|GetUnitDirection(Vector) _returnvalue_5 _returnvalue) (Math|Vector|GetUnitDirection(Vector) _returnvalue_5 _returnvalue_3) (Math|Vector|GetUnitDirection(Vector) _returnvalue_5 _returnvalue_2)))
  (Variables|Default|SetptrArray (Utilities|Array|MakeArray _returnvalue_4 _returnvalue _returnvalue_3 _returnvalue_2))
  (Variables|Default|SetrotArr (Utilities|Array|MakeArray "0, 0, 0" "0,180.000000, 0" "0,90.000000,0.000000" "0.000000,270.000000,0.000000")))

(fn SplitBeam
  (params (input%20beam :type Vector))
  (for _array_element (Variables|Default|GetdirArray)
    (bind _returnvalue (Game|SpawnActorfromClass "/Game/Blueprints/Projectiles/BP_laserPulsePrism.BP_laserPulsePrism_C" (Math|Conversions|ToTransform(Vector) _array_element) "Undefined" 0 0))
    (Variables|/Game/Blueprints/Projectiles/BP_laserPulse.BP_LaserPulse_C|SetSpeed _returnvalue 0.0)
    (Transformation|SetActorLocation _returnvalue (* (Math|Vector|GetUnitDirection(Vector) (Transformation|GetWorldLocation (Variables|Default|GetCube)) _array_element) 1e+02) false false)))

(fn ShootBeams
  (params (speed :type Float%20%28single-precision%29))
  (Effects|SpawnEmitteratLocation "/Game/StarterContent/Particles/P_ShockWave.P_ShockWave" (Transformation|GetWorldLocation (Variables|Default|GetBox)) "0, 0, 0" "3.000000,3.000000,3.000000")
  (for (_array_element _array_index) (Variables|Default|GetptrArray)
    (bind _returnvalue (Game|SpawnActorfromClass "/Game/Blueprints/Projectiles/BP_laserPulsePrism.BP_laserPulsePrism_C" (Math|Transform|MakeTransform (Transformation|GetWorldLocation (Variables|Default|GetBox))) "Undefined" 0 0))
    (Variables|/Game/Blueprints/Projectiles/BP_laserPulse.BP_LaserPulse_C|Setdirection _returnvalue (Utilities|Array|Get(acopy) (Variables|Default|GetdirArray) _array_index))
    (Development|PrintString (Utilities|String|ToString(Float) (stale _output_get)))
    (Transformation|SetActorLocation _returnvalue _array_element false false)
    (Class|Actor|AddActorWorldRotation _returnvalue (Utilities|Array|Get(acopy) (Variables|Default|GetrotArr) _array_index))))

(fn LazerSpawn
  (return 0))