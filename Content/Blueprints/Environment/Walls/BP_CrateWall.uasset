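; Destructible crate wall that explodes when it receives a laser interaction and tells any overlapping actor to destroy its laser.
; LazerInteract is guarded by an Exploded flag, so it only once spawns explosion particles and sound above the actor and destroys the Crate component, leaving the actor itself.
; Powerup spawning is a placeholder that only prints a message, and LazerSpawn is empty.
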(event EventBeginPlay
  (|CallParentFunction) ; This node is disabled and will not be called.\nDrag off pins to build functionality.
)

(event Collision|EventActorBeginOverlap
  (params (OtherActor :type Actor%20Object%20Reference))
  (|CallParentFunction OtherActor)
  (Class|BPIInteractable|LazerDestroy(Message) OtherActor))

(event EventTick
  (params (DeltaSeconds :type Float%20%28single-precision%29))
  (|CallParentFunction DeltaSeconds) ; This node is disabled and will not be called.\nDrag off pins to build functionality.
)

(event EventLazerInteract
  (params (Lazer :type BP%20Laser%20Pulse%20Object%20Reference))
  (if (not (Variables|Default|GetExploded))
    (Variables|Default|SetExploded true)
    (CallFunction|Explode)
    (CallFunction|SpawnPowerup)))

(fn ConstructionScript
  (|CallParentFunction))

(fn Explode
  (bind _returnvalue (Transformation|GetActorLocation))
  (bind _returnvalue_2 (+ _returnvalue "0, 0,50.000000"))
  (Effects|SpawnEmitteratLocation "/Game/StarterContent/Particles/P_Explosion.P_Explosion" _returnvalue_2)
  (Audio|SpawnSoundatLocation "/Game/Audio/SoundWaves/Effect/SW_Explosion_1.SW_Explosion_1" _returnvalue_2 "0, 0, 0" 1.0 1.0 0.0 0 0)
  (Components|DestroyComponent (Variables|Default|GetCrate)))

(fn SpawnPowerup
  (Development|PrintString "CrateWall Placeholder: Spawn Powerup Function"))

(fn LazerSpawn
  (return 0))