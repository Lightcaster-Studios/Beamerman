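; Explosive barrel environment actor that blows up once when hit by a lazer interaction.
; LazerInteract sets an Exploded guard, notifies the lazer via LazerDestroyMessage, spawns BP_BarrelExplosion and calls Explode.
; Explode plays particle and sound effects slightly above the actor, then destroys only the Barrel component, leaving the actor in place.
; A Falling function, not called within this graph, offsets the actor vertically by FallSpeed while tracking remaining Height.
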(event EventLazerInteract
  (params (Lazer :type BP%20Laser%20Pulse%20Object%20Reference))
  (if (not (Variables|Default|GetExploded))
    (Variables|Default|SetExploded true)
    (Class|BPIInteractable|LazerDestroy(Message) Lazer self)
    (Game|SpawnActorfromClass "/Game/Blueprints/Environment/BP_BarrelExplosion.BP_BarrelExplosion_C" (Math|Transform|MakeTransform (Transformation|GetActorLocation) "0, 0, 0" "1,1,1") "Undefined" 0 0)
    (CallFunction|Explode)))

(fn ConstructionScript)

(fn Explode
  (bind _returnvalue (Transformation|GetActorLocation))
  (bind _returnvalue_2 (+ _returnvalue "0, 0,50.000000"))
  (Effects|SpawnEmitteratLocation "/Game/StarterContent/Particles/P_Explosion.P_Explosion" _returnvalue_2)
  (Audio|SpawnSoundatLocation "/Game/Audio/SFX/SW_Explosion_1.SW_Explosion_1" _returnvalue_2 "0, 0, 0" 1.0 1.0 0.0 0 0)
  (Components|DestroyComponent (Variables|Default|GetBarrel)))

(fn Falling
  (if (> (Variables|Default|GetHeight) 0.0)
    (Transformation|AddActorWorldOffset (Math|Vector|MakeVector 0.0 0.0 (Variables|Default|GetFallSpeed)))
    (if (<= (+ (Variables|Default|GetHeight) (Variables|Default|GetFallSpeed)) 0.0)
      (Variables|Default|SetHeight 0.0)
      (else
        (Variables|Default|SetHeight (+ (Variables|Default|GetHeight) (Variables|Default|GetFallSpeed)))))))