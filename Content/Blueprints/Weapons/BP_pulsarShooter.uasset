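; BP_pulsarShooter is a weapon actor that automatically fires a BP_laserPulse from its Sphere every three seconds.
; BeginPlay runs an endless Delay loop that spawns the pulse at the Sphere's world location.
; CalculateForwardVector derives the aim from the Cube-to-Sphere relative locations and feeds it to the pulse's SetDirection, whose result is printed.
; The actor's own SetDirection function is an empty stub.
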(event EventBeginPlay
  (Utilities|FlowControl|Delay 3.0 :!label _label)
  (bind _returnvalue (Game|SpawnActorfromClass "/Game/Blueprints/Projectiles/BP_laserPulse.BP_laserPulse_C" (Math|Conversions|ToTransform(Vector) (Transformation|GetWorldLocation (Variables|Default|GetSphere))) "Undefined" 0 0))
  (bind _fwd_vector (CallFunction|CalculateForwardVector))
  (bind _success (Default|SetDirection _returnvalue _fwd_vector))
  (Development|PrintString (Utilities|String|ToString(Boolean) _success))
  (goto _label))

(event Collision|EventActorBeginOverlap
  (params (OtherActor :type Actor%20Object%20Reference)))

(event EventTick
  (params (DeltaSeconds :type Float%20%28single-precision%29)))

(fn ConstructionScript)

(fn CalculateForwardVector
  (return (Math|Vector|GetUnitDirection(Vector) (Variables|/Script/Engine.SceneComponent|GetRelativeLocation (Variables|Default|GetCube)) (Variables|/Script/Engine.SceneComponent|GetRelativeLocation (Variables|Default|GetSphere)))))

(fn SetDirection
  (params (Direction :type Vector :default "0, 0, 0")))