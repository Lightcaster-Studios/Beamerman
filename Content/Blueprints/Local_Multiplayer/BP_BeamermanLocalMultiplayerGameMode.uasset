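; Game mode for Beamerman local multiplayer, running a player registration stage and then the match.
; Pre-created controllers register on selection platforms; starting spawns humans, plus optional bots in empty slots, at tagged PlayerStarts.
; Each player index gets its own appearance and collision channel, shared through the persistent game instance.
; Deaths are recorded with times, and Tick triggers Defeat when no humans remain or Victory when one human stands alone.
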(event Custom|RegisterDeadPlayer
  (params (DeadPlayer :type BP%20Beamerman%20Player%20Object%20Reference))
  (PlayerDeathRelated|RegisterCharacterDeathHelper DeadPlayer))

(event EventTick
  (params (DeltaSeconds :type Float%20%28single-precision%29))
  (if (not (Variables|PlayerRegistration|GetIsGameAtPlayerRegisterStage))
    (if (== (Utilities|Set|Length (Variables|PlayerLivingStatus|GetAliveHumanPlayers)) 0)
      (EndGameFunctions|Defeat)
      (elif (and (== (Utilities|Set|Length (Variables|PlayerLivingStatus|GetAliveHumanPlayers)) 1) (== (Utilities|Set|Length (Variables|PlayerLivingStatus|GetAliveBots)) 0))
        ;[1 1 1] Add the last human player to the player record
        (bind _result (Utilities|Set|ToArray (Variables|PlayerLivingStatus|GetAliveHumanPlayers)))
        (PlayerDeathRelated|AddPlayerRecord (.Value (Utilities|Map|Find (Variables|General|GetPlayerIndexToPlayerRef) (Utilities|Array|Get(acopy) _result))))
        (EndGameFunctions|Victory)))))

(event Input|ActionEvents|InputActionEscapeMenu
  (params (Key :type Key%20Structure :default "None"))
  (:Pressed
    (if (not (Variables|PlayerRegistration|GetIsGameAtPlayerRegisterStage)) ; If not at player selection, go back to main menu
      (CallFunction|TogglePauseMenu))))

(event Custom|StartGame
  (bind _returnvalue (Game|GetPlayerCameraManager 0))
  (bind _playerregistrationwidgetref (Variables|PlayerRegistration|GetPlayerRegistrationWidgetRef))
  (Components|Animation|PlayAnimation _playerregistrationwidgetref (Variables|/Game/UI/LocalMultiplayerRegistration/LocalMultiplayerPlayerDetectionHUD.LocalMultiplayerPlayerDetectionHUD_C|GetFade _playerregistrationwidgetref) 0.0
    (:then
      (CameraFades|StartCameraFade :self _returnvalue :ToAlpha 1.0 :Duration 1.0 :bHoldWhenFinished true)
      (Utilities|FlowControl|Delay 2.0)
      (CameraFades|StartCameraFade :self _returnvalue :FromAlpha 1.0 :Duration 1.0)
      (Variables|PlayerRegistration|SetIsGameAtPlayerRegisterStage false)
      (PlayerRegistration|SpawnPlayersinMap)
      (if (Variables|General|GetShouldBotsSpawn)
        (PlayerRegistration|SpawnBotsinMap))
      (PlayerRegistration|UpdateGameInstance)
      (PlayerRegistration|SetupPlayerCollisions)
      (PlayerRegistration|SetupGameHUD)
      (Default|PlayGameMusic (Variables|General|GetPersistentGameInstanceRef))
      (Game|Player|SetViewTargetwithBlend (Game|GetPlayerController 0) (Variables|Components|GetGameCamera) 0.0 "VTBlend_EaseOut" 0.0 false))))

(event Custom|UnregisterPlayer
  (params (Player%20Controller :type Player%20Controller%20Object%20Reference))
  (bind _returnvalue (Class|GameplayStatics|GetPlayerControllerID Player%20Controller))
  (if (Variables|PlayerRegistration|GetIsGameAtPlayerRegisterStage)
    (Utilities|Array|RemoveItem (Variables|General|GetHumanPlayerControllers) Player%20Controller)
    (Utilities|Array|SetArrayElem (Variables|PlayerRegistration|GetIsPlayerPresent) _returnvalue false)
    (PlayerRegistration|TogglePlatform _returnvalue false)))

(event Custom|RegisterPlayer
  (params (Player%20Controller :type Player%20Controller%20Object%20Reference))
  (bind _returnvalue (Class|GameplayStatics|GetPlayerControllerID Player%20Controller))
  (if (Variables|PlayerRegistration|GetIsGameAtPlayerRegisterStage)
    (Utilities|Array|AddUnique (Variables|General|GetHumanPlayerControllers) Player%20Controller)
    (Utilities|Array|SetArrayElem (Variables|PlayerRegistration|GetIsPlayerPresent) _returnvalue true)
    (Audio|PlaySound2D "/Game/Audio/SFX/start-game-sfx.start-game-sfx" 1.0 1.0 0.0 0 0)
    (PlayerRegistration|TogglePlatform _returnvalue true)))

(event EventBeginPlay
  (PlayerRegistration|SpawnPlayerControllers)
  (PlayerRegistration|SetupMultiplayerRegistrationHUD)
  (PlayerRegistration|GetAllLevelObjects)
  (bind _aspersistent_game_instance (Utilities|Casting|CastToPersistentGameInstance (Game|GetGameInstance)))
  (bind _output_get (Variables|General|SetPersistentGameInstanceRef _aspersistent_game_instance))
  (Default|PlayMainMenuAudio _output_get))

(fn ConstructionScript)

(fn Defeat
  (Game|SetGamePaused true)
  ;[1 1 1] Disable player controls
  (Variables|/Script/Engine.PlayerController|SetbShowMouseCursor (Game|GetPlayerController 0) true)
  (for _array_element (Variables|General|GetHumanPlayerControllers)
    (Input|DisableInput _array_element)
    (Default|PlayEndGameAudio (Variables|General|GetPersistentGameInstanceRef))
    (bind _returnvalue (UserInterface|CreateWidget "/Game/UI/EndGameDefeat/UI_EndGameDefeat.UI_EndGameDefeat_C" (Game|GetPlayerController 0)))
    (LocalVariables|SetDefeatWidgetRef _returnvalue)
    (bind _returnvalue_2 (Game|GetCurrentLevelName true))
    (Variables|/Game/UI/EndGameDefeat/UI_EndGameDefeat.UI_EndGameDefeat_C|SetCurrentLevelName (LocalVariables|GetDefeatWidgetRef) (Utilities|String|StringToName _returnvalue_2))
    (UserInterface|Viewport|AddtoViewport (LocalVariables|GetDefeatWidgetRef) 0)))

(fn Victory
  (Game|SetGamePaused true)
  ;[1 1 1] Disable player controls
  (Variables|/Script/Engine.PlayerController|SetbShowMouseCursor (Game|GetPlayerController 0) true)
  (for _array_element (Variables|General|GetHumanPlayerControllers)
    (Input|DisableInput _array_element)
    (Default|PlayEndGameAudio (Variables|General|GetPersistentGameInstanceRef))
    (bind _returnvalue (UserInterface|CreateWidget "/Game/UI/EndGameVictory/UI_Victory.UI_Victory_C" (Game|GetPlayerController 0) (Variables|General|GetPlayerRecords)))
    (LocalVariables|SetVictoryWidgetRef _returnvalue)
    (bind _returnvalue_2 (Game|GetCurrentLevelName true))
    (Variables|/Game/UI/EndGameVictory/UI_Victory.UI_Victory_C|SetCurrentLevelName (LocalVariables|GetVictoryWidgetRef) (Utilities|String|StringToName _returnvalue_2))
    (UserInterface|Animation|PlayAnimation (LocalVariables|GetVictoryWidgetRef) (Variables|/Game/UI/EndGameVictory/UI_Victory.UI_Victory_C|GetSlide (LocalVariables|GetVictoryWidgetRef)) 0.0 1 "Forward" 1.0 false)
    (UserInterface|Viewport|AddtoViewport (LocalVariables|GetVictoryWidgetRef) 0)))

(fn SetupPlayerCollisions
  (bind _persistentgameinstanceref (Variables|General|GetPersistentGameInstanceRef))
  (bind _playercollisionmappings (Variables|/Game/PersistentGameInstance.PersistentGameInstance_C|GetPlayerCollisionMappings _persistentgameinstanceref))
  (bind _keys (Utilities|Map|Keys (Variables|General|GetPlayerIndexToPlayerRef)))
  (for _array_element _keys
    (switch int _array_element
      (:0
        (Collision|SetCollisionObjectType (Variables|/Script/Engine.Character|GetCapsuleComponent (.Value (Utilities|Map|Find (Variables|General|GetPlayerIndexToPlayerRef) _array_element))) "ECC_GameTraceChannel1"))
      (:1
        (Collision|SetCollisionObjectType (Variables|/Script/Engine.Character|GetCapsuleComponent (.Value (Utilities|Map|Find (Variables|General|GetPlayerIndexToPlayerRef) _array_element))) "ECC_GameTraceChannel2"))
      (:2
        (Collision|SetCollisionObjectType (Variables|/Script/Engine.Character|GetCapsuleComponent (.Value (Utilities|Map|Find (Variables|General|GetPlayerIndexToPlayerRef) _array_element))) "ECC_GameTraceChannel3"))
      (:3
        (Collision|SetCollisionObjectType (Variables|/Script/Engine.Character|GetCapsuleComponent (.Value (Utilities|Map|Find (Variables|General|GetPlayerIndexToPlayerRef) _array_element))) "ECC_GameTraceChannel4"))))
  (bind _keys_2 (Utilities|Map|Keys (Variables|General|GetPlayerIndexToPlayerRef)))
  (for (_array_element_2 _array_index) _keys_2
    (switch int _array_element_2
      (:0
        (Utilities|Map|Add _playercollisionmappings (.Value (Utilities|Map|Find (Variables|General|GetPlayerIndexToPlayerRef) _array_index)) (Utilities|Enum|LiteralenumECollisionChannel "ECC_GameTraceChannel1")))
      (:1
        (Utilities|Map|Add _playercollisionmappings (.Value (Utilities|Map|Find (Variables|General|GetPlayerIndexToPlayerRef) _array_index)) (Utilities|Enum|LiteralenumECollisionChannel "ECC_GameTraceChannel2")))
      (:2
        (Utilities|Map|Add _playercollisionmappings (.Value (Utilities|Map|Find (Variables|General|GetPlayerIndexToPlayerRef) _array_index)) (Utilities|Enum|LiteralenumECollisionChannel "ECC_GameTraceChannel3")))
      (:3
        (Utilities|Map|Add _playercollisionmappings (.Value (Utilities|Map|Find (Variables|General|GetPlayerIndexToPlayerRef) _array_index)) (Utilities|Enum|LiteralenumECollisionChannel "ECC_GameTraceChannel4"))))))

(fn SetPlayerAppearance
  (params (Player :type BP%20Beamerman%20Player%20Object%20Reference) (Player%20Index :type Integer))
  (bind _mesh (Variables|/Script/Engine.Character|GetMesh Player))
  (Variables|/Game/Blueprints/Player/BP_BeamermanPlayer.BP_BeamermanPlayer_C|SetDroneMaterial Player (Utilities|Array|Get(acopy) (Variables|PlayerAppearance|GetPlayerDroneMaterials) Player%20Index))
  (Variables|/Game/Blueprints/Player/BP_BeamermanPlayer.BP_BeamermanPlayer_C|SetLazerMaterial Player (Utilities|Array|Get(acopy) (Variables|PlayerAppearance|GetPlayerLazerMaterials) Player%20Index))
  (Class|SkinnedMeshComponent|SetSkeletalMesh _mesh (Utilities|Array|Get(acopy) (Variables|PlayerAppearance|GetPlayerSkeletalMeshes) Player%20Index) true)
  (Rendering|Material|SetMaterial _mesh 1 (Utilities|Array|Get(acopy) (Variables|PlayerAppearance|GetPlayerMaterials) Player%20Index)))

(fn UpdateGameInstance
  (bind _aspersistent_game_instance (Utilities|Casting|CastToPersistentGameInstance (Game|GetGameInstance)))
  (Variables|General|SetPersistentGameInstanceRef _aspersistent_game_instance)
  (Variables|/Game/PersistentGameInstance.PersistentGameInstance_C|SetPlayerIndexToPlayerRef (Variables|General|GetPersistentGameInstanceRef) (Variables|General|GetPlayerIndexToPlayerRef))
  (Variables|/Game/PersistentGameInstance.PersistentGameInstance_C|SetHasLocalMultiplayerGameStarted (Variables|General|GetPersistentGameInstanceRef) (not (Variables|PlayerRegistration|GetIsGameAtPlayerRegisterStage))))

(fn GetAllLevelObjects
  (bind _outactors (Actor|GetAllActorsOfClass "/Script/Engine.PlayerStart"))
  (Variables|PlayerRegistration|SetPlayerStartLocations _outactors)
  ;[1 1 1] Get all the controller detection platforms for each player
  (bind _outactors_2 (Actor|GetAllActorsOfClass "/Game/Blueprints/Environment/Multiplayer/ControllerSelectionPlatform.ControllerSelectionPlatform_C"))
  (for _array_element _outactors_2
    (Utilities|Map|Add (Variables|Default|GetPlayer%20Platforms) (Variables|/Game/Blueprints/Environment/Multiplayer/ControllerSelectionPlatform.ControllerSelectionPlatform_C|GetPlatform%20Number _array_element) _array_element)))

(fn SpawnPlayerControllers
  (for _index (range 0 (- (Variables|General|GetMaxPlayers) 1))
    (Class|GameplayStatics|CreatePlayer _index)
    (Utilities|Array|Add (Variables|PlayerRegistration|GetIsPlayerPresent) false)))

(fn SpawnPlayersinMap
  (for _array_element (Variables|General|GetHumanPlayerControllers)
    (bind _output_get (LocalVariables|SetcurPlayerController _array_element))
    (LocalVariables|SetcurPlayerIndex (Class|GameplayStatics|GetPlayerControllerID _output_get))
    ;[1 1 1] Ensures we are spawning the character at the correct spawn point
    (bind _array_element_2 (Utilities|Array|ForEachLoopwithBreak (Variables|PlayerRegistration|GetPlayerStartLocations) :!label _label)
      (:LoopBody
        (bind _output_get_2 (LocalVariables|SetcurPlayerStart _array_element_2))
        (if (Utilities|Name|Equal(Name) (Variables|/Script/Engine.PlayerStart|GetPlayerStartTag _output_get_2) (Utilities|String|StringToName (Utilities|String|ToString(Integer) (LocalVariables|GetcurPlayerIndex))))
          (bind _returnvalue (Game|SpawnActorfromClass "/Game/Blueprints/Player/BP_BeamermanPlayer.BP_BeamermanPlayer_C" (Transformation|GetActorTransform (LocalVariables|GetcurPlayerStart)) "Undefined" 0 (LocalVariables|GetcurPlayerIndex) 0))
          (LocalVariables|SetcurSpawnedPlayer _returnvalue)
          (Pawn|Possess (LocalVariables|GetcurPlayerController) (LocalVariables|GetcurSpawnedPlayer))
          (Game|Player|SetViewTargetwithBlend (LocalVariables|GetcurPlayerController) (Variables|Components|GetGameCamera) 0.0 "VTBlend_Linear" 0.0 false)
          (PlayerRegistration|SetPlayerAppearance (LocalVariables|GetcurSpawnedPlayer) (LocalVariables|GetcurPlayerIndex))
          (Utilities|Map|Add (Variables|General|GetPlayerIndexToPlayerRef) (LocalVariables|GetcurPlayerIndex) (LocalVariables|GetcurSpawnedPlayer))
          (Utilities|Set|Add (Variables|PlayerLivingStatus|GetAliveHumanPlayers) (LocalVariables|GetcurPlayerIndex))
          (goto _label Break))))))

(fn SpawnBotsinMap
  (for (_array_element _array_index) (Variables|PlayerRegistration|GetIsPlayerPresent)
    (LocalVariables|SetcurPlayerIndex _array_index)
    ;[1 1 1] if there isnt a human player at this index
    (if (not _array_element)
      ;[1 1 1] Ensures we are spawning the character at the correct spawn point
      (bind _array_element_2 (Utilities|Array|ForEachLoopwithBreak (Variables|PlayerRegistration|GetPlayerStartLocations) :!label _label)
        (:LoopBody
          (bind _output_get (LocalVariables|SetcurPlayerStart _array_element_2))
          (if (Utilities|Name|Equal(Name) (Variables|/Script/Engine.PlayerStart|GetPlayerStartTag _output_get) (Utilities|String|StringToName (Utilities|String|ToString(Integer) (LocalVariables|GetcurPlayerIndex))))
            (bind _returnvalue (AI|SpawnAIFromClass "/Game/Blueprints/AIPlayer/BP_BeamermanBot.BP_BeamermanBot_C" 0 (.location (Transformation|GetActorTransform (LocalVariables|GetcurPlayerStart))) (.rotation (Transformation|GetActorTransform (LocalVariables|GetcurPlayerStart))) false))
            (bind _asbp_beamerman_player (Utilities|Casting|CastToBP_BeamermanPlayer _returnvalue))
            (LocalVariables|SetcurSpawnedAIPlayer _asbp_beamerman_player)
            (Variables|/Game/Blueprints/Player/BP_BeamermanPlayer.BP_BeamermanPlayer_C|SetPlayerID (LocalVariables|GetcurSpawnedAIPlayer) (LocalVariables|GetcurPlayerIndex))
            (PlayerRegistration|SetPlayerAppearance (LocalVariables|GetcurSpawnedAIPlayer) (LocalVariables|GetcurPlayerIndex))
            (Utilities|Map|Add (Variables|General|GetPlayerIndexToPlayerRef) (LocalVariables|GetcurPlayerIndex) (LocalVariables|GetcurSpawnedAIPlayer))
            (Utilities|Set|Add (Variables|PlayerLivingStatus|GetAliveBots) (LocalVariables|GetcurPlayerIndex))
            (goto _label Break)))))))

(fn SetupMultiplayerRegistrationHUD
  (bind _returnvalue (UserInterface|CreateWidget "/Game/UI/LocalMultiplayerRegistration/LocalMultiplayerPlayerDetectionHUD.LocalMultiplayerPlayerDetectionHUD_C"))
  (bind _output_get (Variables|PlayerRegistration|SetPlayerRegistrationWidgetRef _returnvalue))
  (UserInterface|Viewport|AddtoViewport _output_get 0)
  (Variables|/Script/Engine.PlayerController|SetbShowMouseCursor (Game|GetPlayerController 0) true))

(fn SetupGameHUD
  (Widget|RemovefromParent (Variables|PlayerRegistration|GetPlayerRegistrationWidgetRef))
  (bind _returnvalue (UserInterface|CreateWidget "/Game/UI/HUD/LocalMultiplayerGameWidget.LocalMultiplayerGameWidget_C"))
  (UserInterface|Viewport|AddtoViewport _returnvalue 0))

(fn RegisterCharacterDeathHelper
  (params (Player :type BP%20Beamerman%20Player%20Object%20Reference%20%28by%20ref%29))
  (bind _output_get (LocalVariables|SetDeadPlayerRef Player))
  (PlayerDeathRelated|AddPlayerRecord _output_get)
  (if (== (Utilities|GetClass (LocalVariables|GetDeadPlayerRef)) "/Game/Blueprints/AIPlayer/BP_BeamermanBot.BP_BeamermanBot_C")
    (Utilities|Set|Remove (Variables|PlayerLivingStatus|GetAliveBots) (Variables|/Game/Blueprints/Player/BP_BeamermanPlayer.BP_BeamermanPlayer_C|GetPlayerID (LocalVariables|GetDeadPlayerRef)))
    (else
      (Utilities|Set|Remove (Variables|PlayerLivingStatus|GetAliveHumanPlayers) (Variables|/Game/Blueprints/Player/BP_BeamermanPlayer.BP_BeamermanPlayer_C|GetPlayerID (LocalVariables|GetDeadPlayerRef))))))

(fn AddPlayerRecord
  (params (PlayerRef :type BP%20Beamerman%20Player%20Object%20Reference))
  (bind _persistentgameinstanceref (Variables|General|GetPersistentGameInstanceRef))
  (Utilities|Array|AddUnique (Variables|General|GetPlayerRecords) (Utilities|Struct|MakeStruct_PlayerDeath (Variables|/Game/Blueprints/Player/BP_BeamermanPlayer.BP_BeamermanPlayer_C|GetPlayerID PlayerRef) (- (Variables|/Game/PersistentGameInstance.PersistentGameInstance_C|GetTimeLimit _persistentgameinstanceref) (Variables|/Game/PersistentGameInstance.PersistentGameInstance_C|GetCurrentTimeRemaining _persistentgameinstanceref))))
  (return))

(fn TogglePauseMenu
  (if (Variables|Pause|GetIsPauseMenuOpen)
    (Default|CloseMenu (Variables|Pause|GetPauseMenuWidgetRef))
    (Variables|Pause|SetIsPauseMenuOpen false)
    (else
      (bind _returnvalue (UserInterface|CreateWidget "/Game/UI/PauseMenu/UI_PauseMenuWidget.UI_PauseMenuWidget_C" (Game|GetPlayerController 0)))
      (bind _output_get (Variables|Pause|SetPauseMenuWidgetRef _returnvalue))
      (UserInterface|Viewport|AddtoViewport _output_get 0)
      (Game|SetGamePaused true)
      (Variables|/Script/Engine.PlayerController|SetbShowMouseCursor (Game|GetPlayerController 0) true)
      (Variables|Pause|SetIsPauseMenuOpen true))))

(fn TogglePlatform
  (params (Controller%20ID :type Integer) (Activate? :type Boolean))
  (Default|Toggle (.Value (Utilities|Map|Find (Variables|Default|GetPlayer%20Platforms) Controller%20ID)) Activate?))