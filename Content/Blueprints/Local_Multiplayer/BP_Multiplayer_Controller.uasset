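; BP_Multiplayer_Controller is a controller for local multiplayer that lets each player join or leave the game through input.
; On BeginPlay it casts the game mode to BP_BeamermanLocalMultiplayerGameMode and stores the reference.
; The RegisterPlayer and UnregisterPlayer input actions pass the controller itself to that game mode, which handles the registration.
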(event EventBeginPlay
  (bind _asbp_beamerman_local_multiplayer_game_mode (Utilities|Casting|CastToBP_BeamermanLocalMultiplayerGameMode (Game|GetGameMode)))
  (Variables|Default|SetmultiplayerGameModeRef _asbp_beamerman_local_multiplayer_game_mode))

(event Input|ActionEvents|InputActionRegisterPlayer
  (params (Key :type Key%20Structure))
  (:Pressed
    (Default|RegisterPlayer (Variables|Default|GetmultiplayerGameModeRef) self)))

(event Input|ActionEvents|InputActionUnregisterPlayer
  (params (Key :type Key%20Structure))
  (:Pressed
    (Default|UnregisterPlayer (Variables|Default|GetmultiplayerGameModeRef) self)))

(fn ConstructionScript)