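; Middleman functions that route laser hit and pickup events to the responsible player's ScoreTracker in Beamerman's online scoring.
; Laser hits branch by casting the target to the multiplayer player Blueprint, crediting the laser's owner with either a player hit or an object hit.
; Self-hits score nothing, and a player hit also counts as a kill if the victim is dead.
; Point orb and powerup pickups increment the collecting player's tracker.
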(fn LazerReportHit
  (params (Lazer :type BP%20Laser%20Pulse%20M%20Object%20Reference) (Hit%20Object :type Actor%20Object%20Reference) (Hit%20Component :type Primitive%20Component%20Object%20Reference))
  (bind _asbp_beamerman_multi_player (Utilities|Casting|CastToBP_BeamermanMultiPlayer Hit%20Object)
    (:then
      (Lazer|LazerHandlePlayerHit Lazer _asbp_beamerman_multi_player))
    (:CastFailed
      (Lazer|LazerHandleObjectHit Lazer Hit%20Object Hit%20Component))))

(fn LazerHandlePlayerHit
  (params (Lazer :type BP%20Laser%20Pulse%20M%20Object%20Reference) (Hit%20Player :type BP%20Beamerman%20Multi%20Player%20Object%20Reference))
  (bind _player (Default|GetOwingPlayer Lazer))
  (if (not (== _player Hit%20Player))
    (bind _output_get (LocalVariables|SetFiringPlayerScoreTracker (Variables|/Game/Blueprints/Player/BP_BeamermanMultiPlayer.BP_BeamermanMultiPlayer_C|GetScoreTracker _player)))
    (Default|IncrementPlayerHit _output_get Lazer)
    (if (Variables|/Game/Blueprints/Player/BP_BeamermanMultiPlayer.BP_BeamermanMultiPlayer_C|GetIsDead Hit%20Player)
      (Default|IncrementPlayerKill (LocalVariables|GetFiringPlayerScoreTracker) Hit%20Player))))

(fn LazerHandleObjectHit
  (params (Lazer :type BP%20Laser%20Pulse%20M%20Object%20Reference) (Hit%20Object :type Actor%20Object%20Reference) (Hit%20Component :type Primitive%20Component%20Object%20Reference))
  (bind _player (Default|GetOwingPlayer Lazer))
  (Default|IncrementObjectHit (Variables|/Game/Blueprints/Player/BP_BeamermanMultiPlayer.BP_BeamermanMultiPlayer_C|GetScoreTracker _player) Hit%20Object Hit%20Component Lazer))

(fn PointOrbReportPickup
  (params (Player :type BP%20Beamerman%20Multi%20Player%20Object%20Reference) (PointOrb :type BP%20Point%20Orb%20Object%20Reference))
  (Default|IncrementPickupPointOrb (Variables|/Game/Blueprints/Player/BP_BeamermanMultiPlayer.BP_BeamermanMultiPlayer_C|GetScoreTracker Player) PointOrb))

(fn PowerupReportPickup
  (params (Player :type BP%20Beamerman%20Multi%20Player%20Object%20Reference) (Powerup :type BP%20Power%20Up%20Default%20M%20Object%20Reference))
  (Default|IncrementPickupPowerup (Variables|/Game/Blueprints/Player/BP_BeamermanMultiPlayer.BP_BeamermanMultiPlayer_C|GetScoreTracker Player)))