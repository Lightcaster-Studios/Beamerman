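; Score tracker owned by a player in online multiplayer, awarding points for kills, laser hits with reflection bonuses, object damage and destruction, pickups, and timed passive gain.
; Each event adjusts a category variable by reference through IncrementScore or DecrementScore, which refresh the total and score string via RecomputeScore and SetTotalScore.
; With theft enabled, a kill moves a percentage of the victim's total to the killer and disables the victim's passive gain.
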(event Custom|Event%20PassiveGain
  (Utilities|FlowControl|Delay (Variables|PassiveGain|GetPassiveGainIntervalSeconds))
  (PassiveGain|IncrementPassiveGain)
  (CallFunction|EventPassiveGain))

(event EventBeginPlay
  (Utilities|FlowControl|Delay 3.0)
  (CallFunction|EventPassiveGain))

(fn ConstructionScript)

(fn DecrementStealScore
  (bind _totalscore (Variables|ScoreTypes|GetTotalScore))
  (bind _playerkilltheftpercentage (Variables|PlayerRelated|GetPlayerKillTheftPercentage))
  (bind _returnvalue (* _totalscore _playerkilltheftpercentage))
  (bind _returnvalue_2 (/ _returnvalue 100))
  (HelperFunctions|DecrementScore (Variables|ScoreTypes|GetStolenScore) _returnvalue_2)
  (return _returnvalue_2))

(fn IncrementScore
  (params (ScoreTypeReference :type Integer%20%28by%20ref%29) (PointsGained :type Integer))
  (|SetBy-RefVar ScoreTypeReference (+ ScoreTypeReference PointsGained))
  (bind _newscore (HelperFunctions|SetTotalScore (Utilities|RecomputeScore)))
  (return _newscore))

(fn IncrementPickupPowerup
  (HelperFunctions|IncrementScore (Variables|ScoreTypes|GetPowerupScore) (Variables|ObjectPickup|GetPowerUpGainAmount)))

(fn IncrementPickupPointOrb
  (params (PointOrb :type BP%20Point%20Orb%20M%20Object%20Reference))
  (HelperFunctions|IncrementScore (Variables|ScoreTypes|GetPointOrbScore) (Variables|/Game/Blueprints/Environment/BP_PointOrb_M.BP_PointOrb_M_C|GetScoreValue PointOrb)))

(fn IncrementPickup
  (params (Picked%20Up%20Object :type Actor%20Object%20Reference))
  (bind _asbp_power_up_default_m (Utilities|Casting|CastToBP_PowerUpDefault_M Picked%20Up%20Object)
    (:then
      (PickupGain|IncrementPickupPowerup))
    (:CastFailed
      (bind _asbp_point_orb_m (Utilities|Casting|CastToBP_PointOrb_M _asbp_power_up_default_m))
      (PickupGain|IncrementPickupPointOrb _asbp_point_orb_m))))

(fn IncrementPlayerHit
  (params (Lazer :type BP%20Laser%20Pulse%20M%20Object%20Reference))
  (HelperFunctions|IncrementScore (Variables|ScoreTypes|GetPlayerHitScore) (+ (Variables|PlayerRelated|GetPlayerHitGainAmount) (Utilities|Array|Get(acopy) (Variables|ObjectHit|GetReflectBonusScoreMap) (Variables|/Game/Blueprints/Projectiles/BP_LaserPulse_M.BP_LaserPulse_M_C|GetTimesReflected Lazer)))))

(fn IncrementPlayerKill
  (params (Killed%20Player :type BP%20Beamerman%20Multi%20Player%20Object%20Reference))
  (bind _score_tracker (Variables|/Game/Blueprints/Player/BP_BeamermanMultiPlayer.BP_BeamermanMultiPlayer_C|GetScore%20Tracker Killed%20Player))
  (HelperFunctions|IncrementScore (Variables|ScoreTypes|GetKillScore) (Variables|PlayerRelated|GetPlayerKillGainAmount))
  (if (Variables|PlayerRelated|GetIsScoreTheftEnabled)
    (bind _stolenscore (PlayerGain|DecrementStealScore _score_tracker))
    (HelperFunctions|IncrementScore (Variables|ScoreTypes|GetTheftScore) _stolenscore)
    (Variables|OnlineMultiplayerScoreTracker_C|SetIsPassiveGainEnabled _score_tracker false)))

(fn IncrementPassiveGain
  (if (Variables|PassiveGain|GetIsPassiveGainEnabled)
    (HelperFunctions|IncrementScore (Variables|ScoreTypes|GetPassiveGainScore) (Variables|PassiveGain|GetPassiveGainAmount))))

(fn IncrementObjectHit
  (params (HitObject :type Actor%20Object%20Reference) (HitComponent :type Primitive%20Component%20Object%20Reference) (Lazer :type BP%20Laser%20Pulse%20M%20Object%20Reference))
  (bind _returnvalue (Utilities|GetClass HitObject))
  (bind _objecthitscoremap (Variables|ObjectHit|GetObjectHitScoreMap))
  (bind (_value _returnvalue_2) (Utilities|Map|Find _objecthitscoremap _returnvalue))
  (bind _valid (ObjectGain|CheckValidObject HitObject HitComponent))
  (if _valid
    (if _returnvalue_2
      (HelperFunctions|IncrementScore (Variables|ScoreTypes|GetObjectDamageScore) _value))))

(fn DecrementScore
  (params (ScoreTypeReference :type Integer%20%28by%20ref%29) (PointsLost :type Integer))
  (|SetBy-RefVar ScoreTypeReference (- ScoreTypeReference PointsLost))
  (bind _newscore (HelperFunctions|SetTotalScore (Utilities|RecomputeScore)))
  (return _newscore))

(fn IncrementObjectDestroyed
  (params (DestroyedObject :type Actor%20Object%20Reference))
  (bind _returnvalue (Utilities|GetClass DestroyedObject))
  (bind _objectdestroyscoremap (Variables|ObjectHit|GetObjectDestroyScoreMap))
  (bind (_value _returnvalue_2) (Utilities|Map|Find _objectdestroyscoremap _returnvalue))
  (if _returnvalue_2
    (HelperFunctions|IncrementScore (Variables|ScoreTypes|GetObjectDestroyScore) _value)))

(fn SetTotalScore
  (params (Score :type Integer))
  (bind _output_get (Variables|ScoreTypes|SetTotalScore Score))
  (Variables|ScoreTypes|SetScoreString (Utilities|String|Append "Score: " (Utilities|String|ToString(Integer) _output_get)))
  (return Score))

(fn CheckValidObject
  (params (HitObject :type Actor%20Object%20Reference) (HitComponent :type Primitive%20Component%20Object%20Reference))
  (bind _asbp_crate_wall_m (Utilities|Casting|CastToBP_CrateWall_M HitObject)
    (:then
      (return (not (Variables|/Game/Blueprints/Environment/Tiles/BP_CrateWall_M.BP_CrateWall_M_C|GetDestroyed _asbp_crate_wall_m))))
    (:CastFailed
      (return true))))