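; IndividualScoreTracker keeps one player's score, split into categories such as kills, hits, object damage, pickups, theft and passive gain.
; Increment functions pass category variables by reference to shared helpers that recompute the total and score string.
; Class-keyed maps score objects, and laser reflections add hit bonuses.
; A timer loop grants passive points; score theft on kills transfers a percentage of the victim's total and disables their passive gain.
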(event Custom|Event%20PassiveGain
  (Utilities|FlowControl|Delay (Variables|PassiveGain|GetPassiveGainIntervalSeconds))
  (PassiveGain|IncrementPassiveGain)
  (CallFunction|EventPassiveGain))

(event EventBeginPlay
  (CallFunction|EventPassiveGain))

(fn ConstructionScript)

(fn DecrementStealScore
  (bind _totalscore (Variables|ScoreTypes|GetTotalScore))
  (bind _playerkilltheftpercentage (Variables|PlayerRelated|GetPlayerKillTheftPercentage))
  (bind _returnvalue (* _totalscore _playerkilltheftpercentage))
  (bind _returnvalue_2 (/ _returnvalue 100))
  (HelperFunctions|DecrementScore (Variables|ScoreTypes|GetStolenScore) _returnvalue_2)
  (return _returnvalue_2))

(fn IncrementScore
  (params (ScoreTypeReference :type Integer%20%28by%20ref%29) (PointsGained :type Integer))
  (|SetBy-RefVar ScoreTypeReference (+ ScoreTypeReference PointsGained))
  (bind _newscore (HelperFunctions|SetTotalScore (Utilities|RecomputeScore)))
  (bind _asbp_beamerman_player (Utilities|Casting|CastToBP_BeamermanPlayer (Components|GetOwner)))
  (if (== (Variables|/Game/Blueprints/Player/BP_BeamermanPlayer.BP_BeamermanPlayer_C|GetPlayerID _asbp_beamerman_player) 0)
    (Development|PrintString (Utilities|DebugGetIncrementScoreString PointsGained _newscore) true true "(R=0.000000,G=0.660000,B=1.000000,A=1.000000)" 4.0)
    (return _newscore)))

(fn IncrementPickupPowerup
  (HelperFunctions|IncrementScore (Variables|ScoreTypes|GetPowerupScore) (Variables|ObjectPickup|GetPowerUpGainAmount)))

(fn IncrementPickupPointOrb
  (params (PointOrb :type BP%20Point%20Orb%20Object%20Reference))
  (HelperFunctions|IncrementScore (Variables|ScoreTypes|GetPointOrbScore) (Variables|/Game/Blueprints/Environment/BP_PointOrb.BP_PointOrb_C|GetScoreValue PointOrb)))

(fn IncrementPickup
  (params (Picked%20Up%20Object :type Actor%20Object%20Reference))
  (bind _asbp_power_up_default (Utilities|Casting|CastToBP_PowerUpDefault Picked%20Up%20Object)
    (:then
      (PickupGain|IncrementPickupPowerup))
    (:CastFailed
      (bind _asbp_point_orb (Utilities|Casting|CastToBP_PointOrb _asbp_power_up_default))
      (PickupGain|IncrementPickupPointOrb _asbp_point_orb))))

(fn IncrementPlayerHit
  (params (Lazer :type BP%20Laser%20Pulse%20Object%20Reference))
  (HelperFunctions|IncrementScore (Variables|ScoreTypes|GetPlayerHitScore) (+ (Variables|PlayerRelated|GetPlayerHitGainAmount) (Utilities|Array|Get(acopy) (Variables|ObjectHit|GetReflectBonusScoreMap) (Variables|/Game/Blueprints/Projectiles/BP_laserPulse.BP_LaserPulse_C|GetTimesReflected Lazer)))))

(fn IncrementPlayerKill
  (params (Killed%20Player :type BP%20Beamerman%20Player%20Object%20Reference))
  (bind _scoretracker (Variables|/Game/Blueprints/Player/BP_BeamermanPlayer.BP_BeamermanPlayer_C|GetScoreTracker Killed%20Player))
  (HelperFunctions|IncrementScore (Variables|ScoreTypes|GetKillScore) (Variables|PlayerRelated|GetPlayerKillGainAmount))
  (if (Variables|PlayerRelated|GetIsScoreTheftEnabled)
    (bind _stolenscore (PlayerGain|DecrementStealScore _scoretracker))
    (HelperFunctions|IncrementScore (Variables|ScoreTypes|GetTheftScore) _stolenscore)
    (Variables|IndividualScoreTracker_C|SetIsPassiveGainEnabled _scoretracker false)))

(fn IncrementPassiveGain
  (if (Variables|PassiveGain|GetIsPassiveGainEnabled)
    (HelperFunctions|IncrementScore (Variables|ScoreTypes|GetPassiveGainScore) (Variables|PassiveGain|GetPassiveGainAmount))))

(fn IncrementObjectHit
  (params (HitObject :type Actor%20Object%20Reference) (Lazer :type BP%20Laser%20Pulse%20Object%20Reference))
  (bind _returnvalue (Utilities|GetClass HitObject))
  (bind _objecthitscoremap (Variables|ObjectHit|GetObjectHitScoreMap))
  (bind (_value _returnvalue_2) (Utilities|Map|Find _objecthitscoremap _returnvalue))
  (if _returnvalue_2
    (HelperFunctions|IncrementScore (Variables|ScoreTypes|GetObjectDamageScore) _value)))

(fn DecrementScore
  (params (ScoreTypeReference :type Integer%20%28by%20ref%29) (PointsLost :type Integer))
  (|SetBy-RefVar ScoreTypeReference (- ScoreTypeReference PointsLost))
  (bind _newscore (HelperFunctions|SetTotalScore (Utilities|RecomputeScore)))
  (return _newscore))

(fn IncrementObjectDestroyed
  (params (DestroyedObject :type Actor%20Object%20Reference))
  (bind _returnvalue (Utilities|GetClass DestroyedObject))
  (bind _objectdestroyscoremap (Variables|ObjectHit|GetObjectDestroyScoreMap))
  (bind (_value _returnvalue_2) (Utilities|Map|Find _objectdestroyscoremap _returnvalue))
  (if _returnvalue_2
    (HelperFunctions|IncrementScore (Variables|ScoreTypes|GetObjectDestroyScore) _value)))

(fn SetTotalScore
  (params (Score :type Integer))
  (bind _output_get (Variables|ScoreTypes|SetTotalScore Score))
  (Variables|ScoreTypes|SetScoreString (Utilities|String|Append "Score: " (Utilities|String|ToString(Integer) _output_get)))
  (return Score))