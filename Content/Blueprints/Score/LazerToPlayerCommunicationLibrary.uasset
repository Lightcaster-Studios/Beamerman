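; Blueprint function library that reports laser hits to the score tracker of the player who fired the laser.
; ReportHit casts the hit object to BP_BeamermanPlayer and routes it to player or object handling.
; Player hits increment the hit count, plus a kill credited against the victim if it is already dead.
; Any other object is passed to the tracker as an object hit.
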(fn ReportHit
  (params (Lazer :type BP%20Laser%20Pulse%20Object%20Reference) (Hit%20Object :type Actor%20Object%20Reference))
  (bind _asbp_beamerman_player (Utilities|Casting|CastToBP_BeamermanPlayer Hit%20Object)
    (:then
      (CallFunction|HandlePlayerHit Lazer _asbp_beamerman_player))
    (:CastFailed
      (CallFunction|HandleObjectHit Lazer Hit%20Object))))

(fn HandlePlayerHit
  (params (Lazer :type BP%20Laser%20Pulse%20Object%20Reference) (Hit%20Player :type BP%20Beamerman%20Player%20Object%20Reference))
  (bind _player (Default|GetOwningPlayer Lazer))
  (bind _output_get (LocalVariables|SetFiringPlayerScoreTracker (Variables|/Game/Blueprints/Player/BP_BeamermanPlayer.BP_BeamermanPlayer_C|GetScoreTracker _player)))
  (Default|IncrementPlayerHit _output_get)
  (if (Variables|/Game/Blueprints/Player/BP_BeamermanPlayer.BP_BeamermanPlayer_C|GetIsDead Hit%20Player)
    (Default|IncrementPlayerKill (LocalVariables|GetFiringPlayerScoreTracker) Hit%20Player)))

(fn HandleObjectHit
  (params (Lazer :type BP%20Laser%20Pulse%20Object%20Reference) (Hit%20Object :type Actor%20Object%20Reference))
  (bind _player (Default|GetOwningPlayer Lazer))
  (Default|IncrementObjectHit (Variables|/Game/Blueprints/Player/BP_BeamermanPlayer.BP_BeamermanPlayer_C|GetScoreTracker _player) Hit%20Object))