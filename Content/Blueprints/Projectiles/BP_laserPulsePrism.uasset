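; BP_laserPulsePrism is a laser pulse projectile variant that treats contact with BP_Prism actors as a special case.
; On overlap, a BP_Prism only triggers a placeholder debug print, while any other actor falls through to the parent's overlap handling.
; The construction script runs the parent's, then sets a fixed Range.
; BeginPlay disables overlap events during level streaming without calling the parent, and Tick is disabled.
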(event EventBeginPlay
  (Variables|Default|SetbGenerateOverlapEventsDuringLevelStreaming false))

(event Collision|EventActorBeginOverlap
  (params (OtherActor :type Actor%20Object%20Reference))
  (if (== (Utilities|GetClass OtherActor) "/Game/Blueprints/Environment/Floors/BP_Prism.BP_Prism_C")
    (Development|PrintString "Hello")
    (else
      (|CallParentFunction OtherActor))))

(event EventTick
  (params (DeltaSeconds :type Float%20%28single-precision%29))
  (|CallParentFunction DeltaSeconds) ; This node is disabled and will not be called.\nDrag off pins to build functionality.
)

(fn ConstructionScript
  (|CallParentFunction)
  (Variables|Default|SetRange 3e+02))