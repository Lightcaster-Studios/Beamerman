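; Laser pulse projectile that travels along a direction until its range runs out, passing itself to overlapped actors through a laser interact message.
; A Delay loop started on BeginPlay, rather than Tick, moves it without sweep, orients it to its direction and scales it up logarithmically.
; Brief spawn immunity makes it ignore diagonal mirrors.
; LazerDestroy spawns a spark effect and destroys it.
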(event EventBeginPlay
  (bind _direction (Variables|Default|Getdirection))
  (bind _speed (Variables|Default|GetSpeed))
  (bind _returnvalue (* _direction _speed))
  (Utilities|FlowControl|Delay (Variables|Default|Getdelta) :!label _label)
  (if (Variables|Default|GetSpawnImmune)
    (if (> (Variables|Default|Gettimer) (Variables|Default|Getdelay))
      (Variables|Default|SetSpawnImmune false)
      (else
        (Variables|Default|Settimer (+ (Variables|Default|Gettimer) (Variables|Default|Getdelta))))))
  (Transformation|AddActorWorldOffset _returnvalue)
  (CallFunction|Bloom)
  (CallFunction|Orientate)
  (bind _output_get (Variables|Default|SetRange (- (Variables|Default|GetRange) (Math|Vector|VectorLength _returnvalue))))
  (if (< _output_get 0.0)
    (Actor|DestroyActor)
    (else
      (goto _label))))

(event EventLazerDestroy
  (Effects|SpawnEmitterAttached "/Game/StarterContent/Particles/P_bounceSpark.P_bounceSpark" (Variables|Default|GetSphere) "None")
  (Development|PrintString "hit")
  (Actor|DestroyActor))

(event EventTick
  (params (DeltaSeconds :type Float%20%28single-precision%29)))

(event Collision|EventActorBeginOverlap
  (params (OtherActor :type Actor%20Object%20Reference))
  (if (Variables|Default|GetSpawnImmune)
    (if (not (== (Utilities|GetClass OtherActor) "/Game/Blueprints/Environment/Tiles/BP_MirrorDiagonal.BP_MirrorDiagonal_C"))
      (Class|BPIInteractable|LazerInteract(Message) OtherActor self :!label _label))
    (else
      (goto _label))))

(fn ConstructionScript
  (Variables|Default|SetOriginalRange (Variables|Default|GetRange)))

(fn Orientate
  (Transformation|SetActorRotation (Math|Conversions|RotationFromXVector (Variables|Default|Getdirection))))

(fn Bloom
  (bind _bloom_time (Variables|Default|GetBloom%20Time))
  (if (not (> (Variables|Default|GetBloomTimer) _bloom_time))
    (bind _output_get (Variables|Default|SetBloomTimer (+ (Variables|Default|GetBloomTimer) (Variables|Default|Getdelta))))
    (Transformation|SetActorScale3D (Math|Vector|MakeVector (* (+ (Math|Float|Log (/ _output_get _bloom_time) 1e+01) 1.0) 1.0) (* (+ (Math|Float|Log (/ _output_get _bloom_time) 1e+01) 1.0) 1.0) (* (+ (Math|Float|Log (/ _output_get _bloom_time) 1e+01) 1.0) 1.0)))))

(fn LazerSpawn
  (return))