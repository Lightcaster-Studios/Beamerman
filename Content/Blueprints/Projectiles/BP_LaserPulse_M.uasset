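; Multiplayer laser pulse projectile that self-moves through a recursive Delay loop, growing on a logarithmic bloom until its range runs out.
; Overlaps with non-owners send an interact message and report the hit.
; LazerDestroy plays sound and reflective or obstructive sparks, then deactivates and destroys the pulse.
; SpawnChild creates server-side reflected pulses with one fewer bounce, boosted speed and size, and damage based on reflection count.
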(event OnComponentBeginOverlap(LazerRootCollider)
  (params (OverlappedComponent :type Primitive%20Component%20Object%20Reference) (OtherActor :type Actor%20Object%20Reference) (OtherComp :type Primitive%20Component%20Object%20Reference) (OtherBodyIndex :type Integer) (bFromSweep :type Boolean) (SweepResult :type Hit%20Result%20Structure%20%28by%20ref%29))
  (CallFunction|TriggerHit OtherActor OtherComp))

(event Custom|LazerEventLoop
  (bind _direction (Variables|Misc|GetDirection))
  (bind _speed (Variables|BoostableLazerStats|GetSpeed))
  (bind _returnvalue (* _direction _speed))
  (Utilities|FlowControl|Delay (Variables|LazerStats|GetDelta))
  (if (Variables|Misc|GetSpawnImmune)
    (if (> (Variables|LazerStats|GetTimer) (Variables|LazerStats|GetDelay))
      (Variables|Misc|SetSpawnImmune false)
      (else
        (Variables|LazerStats|SetTimer (+ (Variables|LazerStats|GetTimer) (Variables|LazerStats|GetDelta))))))
  (Transformation|AddActorWorldOffset _returnvalue true)
  (CallFunction|Bloom)
  (CallFunction|Orientate)
  (bind _output_get (Variables|Misc|SetDistanceRemaining (- (Variables|Misc|GetDistanceRemaining) (Math|Vector|VectorLength _returnvalue))))
  (if (< _output_get 0.0)
    (Actor|DestroyActor)
    (else
      (CallFunction|LazerEventLoop))))

(event Custom|TriggerHit
  (params (HitActor :type Actor%20Object%20Reference) (HitComponent :type Primitive%20Component%20Object%20Reference))
  (if (not (== HitActor (Components|GetOwner)))
    (Class|BPIInteractableM|LazerInteract(Message) HitActor self)
    (CallFunction|LazerReportHit self HitActor HitComponent)))

(event Custom|Laser%20Size
  (params (Scale :type Vector))
  ;[1 1 1] Multicast Events
  (Transformation|SetWorldScale3D (Variables|Default|GetLaserVisualComponents) Scale))

(event Custom|Set%20Material
  (params (Material :type Material%20Instance%20Object%20Reference))
  ;[1 1 1] Multicast Events
  (for _array_element (Components|GetChildrenComponents (Variables|Default|GetLaserVisualComponents) true)
    (bind _asprimitive_component (Utilities|Casting|CastToPrimitiveComponent _array_element))
    (Rendering|Material|SetMaterial _asprimitive_component 0 Material)))

(event Custom|BurnoutSpark
  ;[1 1 1] Multicast Events
  (Effects|SpawnEmitteratLocation "/Game/StarterContent/Particles/P_burnoutSpark.P_burnoutSpark" (Transformation|GetWorldLocation (Variables|Default|GetTailCone))))

(event Custom|BounceSpark
  (params (Location :type Vector))
  ;[1 1 1] Multicast Events
  (Effects|SpawnEmitteratLocation "/Game/StarterContent/Particles/P_bounceSpark.P_bounceSpark" Location "0, 0, 0" "2.000000,2.000000,2.000000"))

(event Custom|LazerSound
  ;[1 1 1] Multicast Events
  (Audio|PlaySoundatLocation "/Game/Audio/SFX/LazerHit.LazerHit" (Transformation|GetActorLocation) "0, 0, 0" 1.0 1.0 0.0 0 0 0))

(event Custom|Server%20Child
  (params (NewDirection :type Vector) (SpawnLocation :type Vector) (Owner :type Actor%20Object%20Reference))
  (if (> (Variables|LazerStats|GetRemainingRelfect) 0)
    (bind _returnvalue (Game|SpawnActorfromClass "BP_LaserPulse_M_C" (Math|Conversions|ToTransform(Vector) SpawnLocation) "Undefined" Owner (Game|GetInstigator)))
    (bind _result (Math|Integer|DecrementInt (Variables|LazerStats|GetRemainingRelfect))
      (:%20%20
        (CallFunction|SetLazerParams _returnvalue _result (Variables|LazerStats|GetRange) NewDirection)
        (CallFunction|BoostReflectChild _returnvalue self)))))

(event Custom|Laser%20Direction
  ;[1 1 1] Multicast Events
  (Transformation|SetActorRotation (Math|Conversions|RotationFromXVector (Variables|Misc|GetDirection))))

(event EventBeginPlay
  (CallFunction|LazerEventLoop))

(event EventLazerDestroy
  (params (CollidedActor :type Actor%20Object%20Reference))
  (CallFunction|DestroyLazer CollidedActor)
  (Utilities|FlowControl|Delay 0.2)
  (Actor|DestroyActor))

(fn ConstructionScript
  (Variables|LazerStats|SetRange (Variables|Misc|GetDistanceRemaining))
  (bind _asbp_beamerman_multi_player (Utilities|Casting|CastToBP_BeamermanMultiPlayer (Game|GetInstigator)))
  (CallFunction|SetMaterial (Variables|/Game/Blueprints/Player/BP_BeamermanMultiPlayer.BP_BeamermanMultiPlayer_C|GetLazerMaterial _asbp_beamerman_multi_player)))

(fn SpawnChild
  (params (NewDirection :type Vector) (SpawnLocation :type Vector) (Owner :type Actor%20Object%20Reference))
  (if (Networking|IsServer)
    (CallFunction|ServerChild NewDirection SpawnLocation Owner)))

(fn SetLazerParams
  (params (RemainingReflects :type Integer) (Range :type Float%20%28single-precision%29) (Direction :type Vector))
  (Variables|LazerStats|SetRemainingRelfect RemainingReflects)
  (bind _output_get (Variables|LazerStats|SetRange Range))
  (Variables|Misc|SetDistanceRemaining _output_get)
  (Variables|Misc|SetDirection Direction))

(fn DestroyLazer
  (params (CollidedActor :type Actor%20Object%20Reference))
  (bind _returnvalue (Utilities|GetClass CollidedActor))
  (if (Utilities|Set|Contains (Variables|CollisionSets|GetReflectiveActorClassSet) _returnvalue)
    (CallFunction|BounceSpark (Transformation|GetWorldLocation (Utilities|Array|Get(acopy) (Actor|GetComponentsbyTag CollidedActor "/Script/Engine.StaticMeshComponent" "LazerSpawn"))))
    (elif (Utilities|Set|Contains (Variables|CollisionSets|GetObstructiveActorClassSet) _returnvalue)
      (CallFunction|BurnoutSpark)
      (else
        (Utilities|Casting|CastToBP_BeamermanMultiPlayer CollidedActor))))
  (CallFunction|LazerSound)
  (CallFunction|DeactivateActor))

(fn Orientate
  (CallFunction|LaserDirection))

(fn Bloom
  (bind _bloomtime (Variables|LazerStats|GetBloomTime))
  (if (<= (Variables|LazerStats|GetBloomTimer) _bloomtime)
    (bind _output_get (Variables|LazerStats|SetBloomTimer (+ (Variables|LazerStats|GetBloomTimer) (Variables|LazerStats|GetDelta))))
    (CallFunction|LaserSize (* (Math|Vector|MakeVector (* (+ (Math|Float|Log (/ _output_get _bloomtime) 1e+01) 1.0) 1.0) (* (+ (Math|Float|Log (/ _output_get _bloomtime) 1e+01) 1.0) 1.0) (* (+ (Math|Float|Log (/ _output_get _bloomtime) 1e+01) 1.0) 1.0)) (Variables|BoostableLazerStats|GetSizeScale)))))

(fn SetLazerMaterial
  (params (Material :type Material%20Instance%20Object%20Reference))
  (Rendering|Material|SetMaterial (Variables|Default|GetFrontSphere) 0 Material)
  (Rendering|Material|SetMaterial (Variables|Default|GetTailCone) 0 Material))

(fn GetOwningPlayer
  (bind _asbp_beamerman_multi_player (Utilities|Casting|CastToBP_BeamermanMultiPlayer (Game|GetInstigator)))
  (return _asbp_beamerman_multi_player))

(fn BoostReflectChild
  (params (Parent%20Lazer :type BP%20Laser%20Pulse%20M%20Object%20Reference))
  (Variables|BoostableLazerStats|SetSpeed (+ (Variables|BP_LaserPulse_M_C|GetSpeed Parent%20Lazer) (Variables|BoostableLazerStats|GetSpeedIncrement)))
  (Variables|BoostableLazerStats|SetSizeScale (+ (Variables|BP_LaserPulse_M_C|GetSizeScale Parent%20Lazer) (Variables|BoostableLazerStats|GetSizeScaleIncrement)))
  (Variables|Misc|SetTimesReflected (+ (Variables|BP_LaserPulse_M_C|GetTimesReflected Parent%20Lazer) 1))
  (Variables|BoostableLazerStats|SetDamage (+ (/ (Variables|BP_LaserPulse_M_C|GetTimesReflected Parent%20Lazer) 2) 1)))

(fn DeactivateActor
  (Rendering|SetActorHiddenInGame true)
  (Collision|SetActorEnableCollision false)
  (Actor|Tick|SetActorTickEnabled false))

(fn LazerSpawn
  (return))