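; Explod-o-Mat power-up that drops an explosive barrel onto the level when a Beamerman player overlaps its box.
; On pickup it plays a sound and picks at random between an empty-field drop and a crate-wall drop.
; The crate-wall drop falls back to an empty field unless a random wall is exploded, though the spawn location re-rolls the wall.
; Barrels spawn at a height offset, with a looping timer calling their Falling function.
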(event OnComponentBeginOverlap(Box)
  (params (OverlappedComponent :type Primitive%20Component%20Object%20Reference) (OtherActor :type Actor%20Object%20Reference) (OtherComp :type Primitive%20Component%20Object%20Reference) (OtherBodyIndex :type Integer) (bFromSweep :type Boolean) (SweepResult :type Hit%20Result%20Structure%20%28by%20ref%29))
  (bind _asbp_beamerman_player (Utilities|Casting|CastToBP_BeamermanPlayer OtherActor))
  (CallFunction|TriggerPowerup _asbp_beamerman_player))

(event EventBeginPlay
  (|CallParentFunction))

(fn ConstructionScript
  (|CallParentFunction))

(fn PowerUpEffect
  (params (Player :type BP%20Beamerman%20Player%20Object%20Reference))
  (Audio|PlaySoundatLocation "/Game/Audio/SFX/PowerUpPickup.PowerUpPickup" (Transformation|GetActorLocation) "0, 0, 0" 1.0 1.0 0.0 0 0 0)
  (if (== (Math|Random|RandomInteger 2) 0)
    (CallFunction|DroponEmptyField)
    (else
      (CallFunction|DroponCrateWall))))

(fn DroponCrateWall
  (bind _outactors (Actor|GetAllActorsOfClass "/Game/Blueprints/Environment/Tiles/BP_CrateWall.BP_CrateWall_C"))
  (if (Variables|/Game/Blueprints/Environment/Tiles/BP_CrateWall.BP_CrateWall_C|GetExploded (Utilities|Array|Get(acopy) _outactors (Math|Random|RandomInteger (Utilities|Array|Length _outactors))))
    (bind _returnvalue (Game|SpawnActorfromClass "/Game/Blueprints/Environment/BP_ExplosiveBarrel.BP_ExplosiveBarrel_C" (Math|Transform|MakeTransform (+ (Transformation|GetActorLocation (Utilities|Array|Get(acopy) _outactors (Math|Random|RandomInteger (Utilities|Array|Length _outactors)))) (Math|Vector|MakeVector 0.0 0.0 (Variables|Default|GetHeight))) "0, 0, 0" "1,1,1") "Undefined" 0 0))
    (Utilities|Time|SetTimerbyFunctionName _returnvalue "Falling" 0.03 true)
    (else
      (CallFunction|DroponEmptyField))))

(fn DroponEmptyField
  (bind _outactors (Actor|GetAllActorsOfClass "/Game/Blueprints/Environment/Tiles/BP_EmptyField.BP_EmptyField_C"))
  (bind _returnvalue (Game|SpawnActorfromClass "/Game/Blueprints/Environment/BP_ExplosiveBarrel.BP_ExplosiveBarrel_C" (Math|Transform|MakeTransform (+ (Transformation|GetActorLocation (Utilities|Array|Get(acopy) _outactors (Math|Random|RandomInteger (Utilities|Array|Length _outactors)))) (Math|Vector|MakeVector 0.0 0.0 (Variables|Default|GetHeight))) "0, 0, 0" "1,1,1") "Undefined" 0 0))
  (Utilities|Time|SetTimerbyFunctionName _returnvalue "Falling" 0.03 true))