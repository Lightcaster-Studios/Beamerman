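; Base multiplayer power-up pickup that faces player 0's camera, plays a sound on BeginPlay and bobs vertically via a timeline.
; TriggerPowerup casts the given actor to BP_BeamermanMultiPlayer, calls the effect function and destroys the pickup.
; The effect is a debug-print placeholder for child Blueprints to override.
; The Box overlap event is empty, so nothing in this Blueprint calls TriggerPowerup.
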(event OnComponentBeginOverlap(Box)
  (params (OverlappedComponent :type Primitive%20Component%20Object%20Reference) (OtherActor :type Actor%20Object%20Reference) (OtherComp :type Primitive%20Component%20Object%20Reference) (OtherBodyIndex :type Integer) (bFromSweep :type Boolean) (SweepResult :type Hit%20Result%20Structure%20%28by%20ref%29)))

(event EventBeginPlay
  (CallFunction|OrientCamera)
  (bind _output_get (Variables|Default|SetOrigin (Transformation|GetActorLocation)))
  (Audio|PlaySoundatLocation "/Game/Audio/SFX/PowerUpPickup.PowerUpPickup" _output_get "0, 0, 0" 1.0 1.0 0.0 0 0 0)
  (bind _floatfactor (Timeline|FloatFactor PlayFromStart)
    (:Update
      (CallFunction|BobbingMotion _floatfactor))))

(fn ConstructionScript)

(fn TriggerPowerup
  (params (OverlappedActor :type Actor%20Object%20Reference))
  (bind _asbp_beamerman_multi_player (Utilities|Casting|CastToBP_BeamermanMultiPlayer OverlappedActor))
  (CallFunction|PowerUpEffectS _asbp_beamerman_multi_player)
  (Actor|DestroyActor))

(fn PowerUpEffectS
  (params (Player :type BP%20Beamerman%20Multi%20Player%20Object%20Reference))
  ;[1 1 1] To Be Implemented in Child
  (Development|PrintString "DEBUG: PowerUpDefault Effect Called"))

(fn OrientCamera
  (bind _returnvalue (Game|GetPlayerController 0))
  (bind _playercameramanager (Variables|/Script/Engine.PlayerController|GetPlayerCameraManager _returnvalue))
  (bind _returnvalue_2 (Camera|GetCameraRotation _playercameramanager))
  (Transformation|SetActorRotation (Math|Rotator|MakeRotationfromAxes (* (Math|Vector|GetForwardVector _returnvalue_2) -1) (* (Math|Vector|GetRightVector _returnvalue_2) -1) (Math|Vector|GetUpVector _returnvalue_2))))

(fn BobbingMotion
  (params (FloatFactor :type Float%20%28single-precision%29))
  (Transformation|SetActorLocation (+ (* "0, 0,30.000000" FloatFactor) (Variables|Default|GetOrigin)) false false))