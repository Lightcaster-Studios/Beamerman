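; Multiplayer power-up pickup that increases the drone count of the Beamerman player who touches it.
; A box overlap casts the other actor to BP_BeamermanMultiPlayer, then triggers the power-up and reports the pickup with the player and itself.
; The PowerUpEffect_S override calls IncreaseDroneCount on the player and plays the pickup sound at the actor's location.
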(event OnComponentBeginOverlap(Box)
  (params (OverlappedComponent :type Primitive%20Component%20Object%20Reference) (OtherActor :type Actor%20Object%20Reference) (OtherComp :type Primitive%20Component%20Object%20Reference) (OtherBodyIndex :type Integer) (bFromSweep :type Boolean) (SweepResult :type Hit%20Result%20Structure%20%28by%20ref%29))
  (bind _asbp_beamerman_multi_player (Utilities|Casting|CastToBP_BeamermanMultiPlayer OtherActor))
  (CallFunction|TriggerPowerup _asbp_beamerman_multi_player)
  (CallFunction|PowerUpReport _asbp_beamerman_multi_player))

(event Custom|PowerUp%20Report
  (params (Player :type BP%20Beamerman%20Multi%20Player%20Object%20Reference))
  (CallFunction|PowerupReportPickup Player self))

(event EventBeginPlay
  (|CallParentFunction))

(fn ConstructionScript
  (|CallParentFunction))

(fn PowerUpEffectS
  (params (Player :type BP%20Beamerman%20Multi%20Player%20Object%20Reference))
  (Default|IncreaseDroneCount Player)
  (Audio|PlaySoundatLocation "/Game/Audio/SFX/PowerUpPickup.PowerUpPickup" (Transformation|GetActorLocation) "0, 0, 0" 1.0 1.0 0.0 0 0 0))