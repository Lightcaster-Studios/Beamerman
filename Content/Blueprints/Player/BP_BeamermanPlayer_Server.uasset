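; Top-down Beamerman player character that moves with optional axis lock and spawns laser-firing drones from a recharging supply, blocked where a drone occupies the grid-snapped spot.
; Input and laser-hit handlers call Forward, Right, Fire and Interact events, then repeat their logic inline.
; Hits pass through exclusive timed armors, one reflecting lasers, before costing health, with flashing invulnerability afterward.
; Power-ups upgrade stats with billboards; death moves the pawn away and notifies the game mode.
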(event Custom|Interact
  (params (Lazer :type BP%20Laser%20Pulse%20Object%20Reference))
  ;[1 1 1] Lazer Hit Behaviors
  (if (not (Variables|TemporaryEffects|GetInvulnerable))
    (if (Variables|TemporaryEffects|GetIsTempArmorActive)
      (CallFunction|TempArmorHit Lazer)
      (elif (Variables|TemporaryEffects|GetIsGlassArmorActive)
        (CallFunction|GlassArmorHit)
        (elif (Variables|TemporaryEffects|GetIsMirroredArmorActive)
          (CallFunction|MirroredArmorHit Lazer)
          (else
            (CallFunction|NormalHit Lazer)))))))

(event Custom|NormalHit
  (params (Lazer :type BP%20Laser%20Pulse%20Object%20Reference))
  ;[1 1 1] Lazer Hit Behaviors
  (CallFunction|TakeDamage)
  (CallFunction|EnableInvulnerabilityFrame)
  (CallFunction|InvulnerabilityFlash)
  (CallFunction|PlayDamageEffects)
  (Class|BPIInteractable|LazerDestroy(Message) Lazer self)
  (Utilities|Time|SetTimerbyFunctionName 0 "DisableInvulnerabilityFrame" (Variables|TemporaryEffects|GetIFrameDuration))
  (if (<= (Variables|IncrementablePlayerStats|GetHealth) 0)
    (CallFunction|Die)))

(event Custom|GlassArmorHit
  ;[1 1 1] Lazer Hit Behaviors
  (bind _output_get (Variables|TemporaryEffects|SetIsGlassArmorActive false))
  (CallFunction|EnableInvulnerabilityFrame)
  (CallFunction|InvulnerabilityFlash)
  (Utilities|Time|SetTimerbyFunctionName 0 "DisableInvulnerabilityFrame" (Variables|TemporaryEffects|GetIFrameShortDuration))
  (CallFunction|TempPowerUpEffect _output_get "/Game/Blueprints/Effects/BP_Effect_MirroredArmor.BP_Effect_MirroredArmor_C"))

(event Custom|InvulnerabilityFlash
  (bind _mesh (Variables|Character|GetMesh))
  ;[1 1 1] Flashing Effect for IFrame
  (if (Variables|TemporaryEffects|GetInvulnerable)
    (Rendering|ToggleVisibility _mesh false)
    (Utilities|Time|SetTimerbyEvent (delegate Custom|InvulnerabilityFlash) 0.1)
    (else
      (Rendering|SetVisibility _mesh true false))))

(event Custom|TempArmorHit
  (params (Lazer :type BP%20Laser%20Pulse%20Object%20Reference))
  ;[1 1 1] Lazer Hit Behaviors
  (bind _output_get (Variables|TemporaryEffects|SetIsTempArmorActive false))
  (CallFunction|EnableInvulnerabilityFrame)
  (CallFunction|InvulnerabilityFlash)
  (Class|BPIInteractable|LazerDestroy(Message) Lazer self)
  (Utilities|Time|SetTimerbyFunctionName 0 "DisableInvulnerabilityFrame" (Variables|TemporaryEffects|GetIFrameShortDuration))
  (CallFunction|TempPowerUpEffect _output_get "/Game/Blueprints/Effects/BP_Effect_TempArmor.BP_Effect_TempArmor_C"))

(event Custom|AIBotFireLazer
  ;[1 1 1] Weapon Firing (Spawn Drone)
)

(event Custom|MirroredArmorHit
  (params (Lazer :type BP%20Laser%20Pulse%20Object%20Reference))
  (bind _self self)
  ;[1 1 1] Lazer Hit Behaviors
  (bind _output_get (Variables|TemporaryEffects|SetIsMirroredArmorActive false))
  (CallFunction|EnableInvulnerabilityFrame)
  (CallFunction|InvulnerabilityFlash)
  (Math|Integer|IncrementInt (Variables|/Game/Blueprints/Projectiles/BP_laserPulse.BP_LaserPulse_C|GetReflectIndex Lazer)
    (:%20%20
      (Default|SpawnChild Lazer (* (Variables|/Game/Blueprints/Projectiles/BP_laserPulse.BP_LaserPulse_C|Getdirection Lazer) -1) (Transformation|GetActorLocation) _self)
      (Class|BPIInteractable|LazerDestroy(Message) Lazer _self)
      (Utilities|Time|SetTimerbyFunctionName 0 "DisableInvulnerabilityFrame" (Variables|TemporaryEffects|GetIFrameShortDuration))
      (CallFunction|TempPowerUpEffect _output_get "/Game/Blueprints/Effects/BP_Effect_GlassArmor.BP_Effect_GlassArmor_C"))))

(event Custom|Forward
  (params (AxisValue :type Float%20%28single-precision%29))
  ;[1 1 1] Axis-locked Movement input
  (if (Variables|CharacterMovement|GetIsAxisLocked)
    (if (not (Variables|CharacterMovement|GetIsMovingRight))
      (if (!= AxisValue 0.0)
        (Variables|CharacterMovement|SetIsMovingForward true)
        (else
          (Variables|CharacterMovement|SetIsMovingForward false)))
      (Pawn|Input|AddMovementInput "1.000000,0.000000, 0" AxisValue false :!label _label))
    (else
      (goto _label))))

(event Custom|Right
  (params (AxisValue :type Float%20%28single-precision%29))
  ;[1 1 1] Axis-locked Movement input
  (if (Variables|CharacterMovement|GetIsAxisLocked)
    (if (not (Variables|CharacterMovement|GetIsMovingForward))
      (if (!= AxisValue 0.0)
        (Variables|CharacterMovement|SetIsMovingRight true)
        (else
          (Variables|CharacterMovement|SetIsMovingRight false)))
      (Pawn|Input|AddMovementInput "0.000000,1.000000,0.000000" AxisValue false :!label _label))
    (else
      (goto _label))))

(event Custom|Fire
  ;[1 1 1] Weapon Firing (Spawn Drone)
  (bind _isvalid (CallFunction|TestValidSpawnLocation))
  (if (and _isvalid (> (Variables|IncrementablePlayerStats|GetNumDrones) 0))
    (Math|Integer|DecrementInt (Variables|IncrementablePlayerStats|GetNumDrones)
      (:%20%20
        (CallFunction|PlayDroneSpawnSFX)
        (CallFunction|SpawnDrone)
        (Utilities|FlowControl|Delay (Variables|FixedPlayerStats|GetDroneRechargeInteval) :!label _label)
        (bind _drone_capacity_reached (CallFunction|DroneRecharge))
        (if (not _drone_capacity_reached)
          (goto _label))))))

(event EventBeginPlay
  ;[1 1 1] Begin Play
  (CallFunction|DroneRecharge)
  (CallFunction|CalculateandSetMaxSpeedandRange)
  (Components|Activation|SetActive (Variables|Default|GetTopDownCamera) true false))

(event EventLazerInteract
  (params (Lazer :type BP%20Laser%20Pulse%20Object%20Reference))
  ;[1 1 1] Lazer Hit Behaviors
  (CallFunction|Interact Lazer)
  (if (not (Variables|TemporaryEffects|GetInvulnerable))
    (if (Variables|TemporaryEffects|GetIsTempArmorActive)
      (CallFunction|TempArmorHit Lazer)
      (elif (Variables|TemporaryEffects|GetIsGlassArmorActive)
        (CallFunction|GlassArmorHit)
        (elif (Variables|TemporaryEffects|GetIsMirroredArmorActive)
          (CallFunction|MirroredArmorHit Lazer)
          (else
            (CallFunction|NormalHit Lazer)))))))

(event Input|ActionEvents|InputActionFireLaser
  (params (Key :type Key%20Structure :default "None"))
  ;[1 1 1] Weapon Firing (Spawn Drone)
  (:Pressed
    (CallFunction|Fire)
    (bind _isvalid (CallFunction|TestValidSpawnLocation))
    (if (and _isvalid (> (Variables|IncrementablePlayerStats|GetNumDrones) 0))
      (Math|Integer|DecrementInt (Variables|IncrementablePlayerStats|GetNumDrones)
        (:%20%20
          (CallFunction|PlayDroneSpawnSFX)
          (CallFunction|SpawnDrone)
          (Utilities|FlowControl|Delay (Variables|FixedPlayerStats|GetDroneRechargeInteval) :!label _label)
          (bind _drone_capacity_reached (CallFunction|DroneRecharge))
          (if (not _drone_capacity_reached)
            (goto _label)))))))

(event Input|AxisEvents|InputAxisMoveForward
  (params (AxisValue :type Float%20%28single-precision%29))
  ;[1 1 1] Axis-locked Movement input
  (CallFunction|Forward AxisValue)
  (if (Variables|CharacterMovement|GetIsAxisLocked)
    (if (not (Variables|CharacterMovement|GetIsMovingRight))
      (if (!= AxisValue 0.0)
        (Variables|CharacterMovement|SetIsMovingForward true)
        (else
          (Variables|CharacterMovement|SetIsMovingForward false)))
      (Pawn|Input|AddMovementInput "1.000000,0.000000, 0" AxisValue false :!label _label))
    (else
      (goto _label))))

(event Input|AxisEvents|InputAxisMoveRight
  (params (AxisValue :type Float%20%28single-precision%29))
  ;[1 1 1] Axis-locked Movement input
  (CallFunction|Right AxisValue)
  (if (Variables|CharacterMovement|GetIsAxisLocked)
    (if (not (Variables|CharacterMovement|GetIsMovingForward))
      (if (!= AxisValue 0.0)
        (Variables|CharacterMovement|SetIsMovingRight true)
        (else
          (Variables|CharacterMovement|SetIsMovingRight false)))
      (Pawn|Input|AddMovementInput "0.000000,1.000000,0.000000" AxisValue false :!label _label))
    (else
      (goto _label))))

(event Custom|MirroredArmor
  (CallFunction|ResetTempPowerUp)
  (bind _output_get (Variables|TemporaryEffects|SetIsMirroredArmorActive true))
  (CallFunction|TempPowerUpEffect _output_get "/Game/Blueprints/Effects/BP_Effect_MirroredArmor.BP_Effect_MirroredArmor_C")
  (CallFunction|SpawnBillboard "MirroredArmor!")
  (Utilities|FlowControl|RetriggerableDelay (Variables|TemporaryEffects|GetTemporaryArmorsDuration))
  (if (Variables|TemporaryEffects|GetIsMirroredArmorActive)
    (bind _output_get_2 (Variables|TemporaryEffects|SetIsMirroredArmorActive false))
    (CallFunction|TempPowerUpEffect _output_get_2 "/Game/Blueprints/Effects/BP_Effect_MirroredArmor.BP_Effect_MirroredArmor_C")))

(event Custom|IncreaseSpeed
  (if (<= (+ (Variables|IncrementablePlayerStats|GetMovementSpeed) (Variables|IncrementValues|GetMovement%20Speed%20Increment%20Value)) (Variables|IncrementablePlayerStats|GetMaxMovementSpeed))
    (bind _output_get (Variables|IncrementablePlayerStats|SetMovementSpeed (+ (Variables|IncrementablePlayerStats|GetMovementSpeed) (Variables|IncrementValues|GetMovement%20Speed%20Increment%20Value))))
    (Variables|/Script/Engine.CharacterMovementComponent|SetMaxWalkSpeed (Variables|Character|GetCharacterMovement) _output_get)
    (Math|Integer|IncrementInt (Variables|IncrementablePlayerStats|GetSpeed%20Level)
      (:%20%20
        (CallFunction|SpawnBillboard "Speed++")))))

(event Custom|TempPowerUpEffect
  (params (IsActive :type Boolean) (EffectClass :type Actor%20Class%20Reference))
  (bind _mesh (Variables|Character|GetMesh))
  ;[1 1 1] For Creating/Destroying Temp Power Up Effect
  (if IsActive
    (bind _returnvalue (Game|SpawnActorfromClass EffectClass (Math|Transform|MakeTransform (Transformation|GetWorldLocation _mesh) "0, 0, 0" "1,1,1") "Undefined" 0 0))
    (Transformation|AttachComponentToComponent (Variables|/Script/Engine.Actor|GetRootComponent _returnvalue) _mesh "None" "SnapToTarget" "KeepRelative" "KeepRelative" true)
    (else
      (Actor|DestroyActor _returnvalue))))

(event Custom|IncreaseReflectCount
  (bind _reflectlevel (Variables|IncrementablePlayerStats|GetReflectLevel))
  (if (< _reflectlevel (Variables|IncrementablePlayerStats|GetMaxReflectLevel))
    (Math|Integer|IncrementInt _reflectlevel
      (:%20%20
        (CallFunction|SpawnBillboard "Reflect++")))))

(event Custom|IncreaseDroneCount
  (bind _dronecapacity (Variables|IncrementablePlayerStats|GetDroneCapacity))
  (if (< _dronecapacity (Variables|IncrementablePlayerStats|GetMaxDroneCapacity))
    (Math|Integer|IncrementInt _dronecapacity
      (:%20%20
        (Math|Integer|IncrementInt (Variables|IncrementablePlayerStats|GetNumDrones)
          (:%20%20
            (CallFunction|SpawnBillboard "DroneCount++")))))))

(event Custom|IncreaseRange
  (if (<= (+ (Variables|IncrementablePlayerStats|GetLazerRange) (Variables|IncrementValues|GetLazer%20Range%20Increment%20Value)) (Variables|IncrementablePlayerStats|GetMaxLazerRange))
    (Variables|IncrementablePlayerStats|SetLazerRange (+ (Variables|IncrementablePlayerStats|GetLazerRange) (Variables|IncrementValues|GetLazer%20Range%20Increment%20Value)))
    (Math|Integer|IncrementInt (Variables|IncrementablePlayerStats|GetRange%20Level)
      (:%20%20
        (CallFunction|SpawnBillboard "Range++")))))

(event Custom|TempArmor
  (CallFunction|ResetTempPowerUp)
  (bind _output_get (Variables|TemporaryEffects|SetIsTempArmorActive true))
  (CallFunction|TempPowerUpEffect _output_get "/Game/Blueprints/Effects/BP_Effect_TempArmor.BP_Effect_TempArmor_C")
  (CallFunction|SpawnBillboard "TempArmor!")
  (Utilities|FlowControl|RetriggerableDelay (Variables|TemporaryEffects|GetTemporaryArmorsDuration))
  (if (Variables|TemporaryEffects|GetIsTempArmorActive)
    (bind _output_get_2 (Variables|TemporaryEffects|SetIsTempArmorActive false))
    (CallFunction|TempPowerUpEffect _output_get_2 "/Game/Blueprints/Effects/BP_Effect_TempArmor.BP_Effect_TempArmor_C")))

(event Custom|ResetTempPowerUp
  ;[1 1 1] Resets Any Active Temp Power Up, Preventing Concurrent Temp Power Ups
  (if (Math|Boolean|ORBoolean (Variables|TemporaryEffects|GetIsTempArmorActive) (Variables|TemporaryEffects|GetIsGlassArmorActive) (Variables|TemporaryEffects|GetIsMirroredArmorActive))
    (if (Variables|TemporaryEffects|GetIsTempArmorActive)
      (bind _output_get (Variables|TemporaryEffects|SetIsTempArmorActive false))
      (CallFunction|TempPowerUpEffect _output_get "/Game/Blueprints/Effects/BP_Effect_TempArmor.BP_Effect_TempArmor_C")
      (elif (Variables|TemporaryEffects|GetIsGlassArmorActive)
        (bind _output_get_2 (Variables|TemporaryEffects|SetIsGlassArmorActive false))
        (CallFunction|TempPowerUpEffect _output_get_2 "/Game/Blueprints/Effects/BP_Effect_GlassArmor.BP_Effect_GlassArmor_C")
        (elif (Variables|TemporaryEffects|GetIsMirroredArmorActive)
          (bind _output_get_3 (Variables|TemporaryEffects|SetIsMirroredArmorActive false))
          (CallFunction|TempPowerUpEffect _output_get_3 "/Game/Blueprints/Effects/BP_Effect_MirroredArmor.BP_Effect_MirroredArmor_C"))))))

(event Custom|GlassArmor
  (CallFunction|ResetTempPowerUp)
  (bind _output_get (Variables|TemporaryEffects|SetIsGlassArmorActive true))
  (CallFunction|TempPowerUpEffect _output_get "/Game/Blueprints/Effects/BP_Effect_GlassArmor.BP_Effect_GlassArmor_C")
  (CallFunction|SpawnBillboard "GlassArmor!")
  (Utilities|FlowControl|RetriggerableDelay (Variables|TemporaryEffects|GetTemporaryArmorsDuration))
  (if (Variables|TemporaryEffects|GetIsGlassArmorActive)
    (bind _output_get_2 (Variables|TemporaryEffects|SetIsGlassArmorActive false))
    (CallFunction|TempPowerUpEffect _output_get_2 "/Game/Blueprints/Effects/BP_Effect_GlassArmor.BP_Effect_GlassArmor_C")))

(fn ConstructionScript
  (Variables|/Script/Engine.CharacterMovementComponent|SetMaxWalkSpeed (Variables|Character|GetCharacterMovement) (Variables|IncrementablePlayerStats|GetMovementSpeed)))

(fn PlayDroneSpawnSFX)

(fn SpawnDrone
  (bind _dronespawnpoint (Variables|Default|GetDroneSpawnPoint))
  (bind _returnvalue (Transformation|GetWorldTransform _dronespawnpoint))
  (bind _returnvalue_2 (Game|SpawnActorfromClass "/Game/Blueprints/Player/BP_LazerDrone.BP_LazerDrone_C" (Math|Transform|MakeTransform (.location _returnvalue) (.rotation _returnvalue) "1,1,1") "AlwaysSpawn" self 0))
  (Default|FireWeapon _returnvalue_2 (Variables|IncrementablePlayerStats|GetReflectLevel) (Variables|IncrementablePlayerStats|GetLazerRange) (Variables|FixedPlayerStats|GetWeaponChargeUpTime)))

(fn TakeDamage
  (Math|Integer|DecrementInt (Variables|IncrementablePlayerStats|GetHealth)))

(fn PlayDamageEffects
  (bind _mesh (Variables|Character|GetMesh))
  (bind _mesh_2 (Variables|Character|GetMesh))
  (bind _returnvalue (Transformation|GetWorldLocation _mesh))
  (bind _returnvalue_2 (Transformation|GetWorldLocation _mesh_2))
  (Effects|SpawnEmitteratLocation "/Game/StarterContent/Particles/P_ShockWave.P_ShockWave" (Math|Vector|MakeVector (.x _returnvalue) (.y _returnvalue) 8e+01))
  (Game|SpawnActorfromClass "/Game/Blueprints/Player/BP_Ghost.BP_Ghost_C" (Math|Transform|MakeTransform _returnvalue_2 "0, 0, 0" "1,1,1") "Undefined" 0 0)
  (Audio|PlaySoundatLocation "/Game/Audio/SFX/PlayerHit.PlayerHit" _returnvalue_2 "0, 0, 0" 1.0 1.0 0.0 0 0 0))

(fn EnableInvulnerabilityFrame
  (Variables|TemporaryEffects|SetInvulnerable true))

(fn DisableInvulnerabilityFrame
  (Variables|TemporaryEffects|SetInvulnerable false))

(fn Die
  (bind _mesh (Variables|Character|GetMesh))
  (bind _returnvalue (Transformation|GetWorldLocation _mesh))
  (if (not (Variables|FixedPlayerStats|GetIsDead))
    (Variables|FixedPlayerStats|SetIsDead true)
    ;[1 1 1] Necessary as some deaths are not triggered by health falling to 0
    (Variables|IncrementablePlayerStats|SetHealth 0)
    (Effects|SpawnEmitteratLocation "/Game/StarterContent/Particles/P_Smoke.P_Smoke" (Math|Vector|MakeVector (.x _returnvalue) (.y _returnvalue) 0.0))
    (Audio|PlaySoundatLocation "/Game/Audio/SFX/PlayerDie.PlayerDie" (Transformation|GetActorLocation) "0, 0, 0" 1.0 1.0 0.0 0 0 0)
    ;[1 1 1] Hacky Death Implementation
    (Transformation|SetActorLocation "5000.000000, 0,-500.000000" false false)
    (Pawn|Components|CharacterMovement|SetMovementMode (Variables|Character|GetCharacterMovement) "MOVE_None" 0)
    (bind _asbp_beamerman_game_mode (Utilities|Casting|CastToBP_BeamermanGameMode (Game|GetGameMode)))
    (Default|PlayerDies _asbp_beamerman_game_mode self)))

(fn SpawnBillboard
  (params (Text :type Text))
  (bind _returnvalue (Game|SpawnActorfromClass "/Game/Blueprints/Misc/BP_Billboard.BP_Billboard_C" (Math|Transform|MakeTransform (Transformation|GetActorLocation) "0, 0, 0" "2.000000,2.000000,2.000000") "Undefined" 0 0))
  (Default|SetText _returnvalue Text))

(fn TestValidSpawnLocation
  (bind _returnvalue (Transformation|GetActorLocation))
  (bind _roundedlocation (Utilities|XYLocationtoNearest _returnvalue 100))
  (bind (_outhit _returnvalue_2) (Collision|LineTraceByChannel (Math|Vector|MakeVector (.x _roundedlocation) (.y _roundedlocation) 1e+01) (Math|Vector|MakeVector (.x _roundedlocation) (.y _roundedlocation) 1.5e+02) "TraceTypeQuery1" false 0 "None"))
  (if _returnvalue_2
    (Utilities|Casting|CastToBP_LazerDrone (.HitActor (Collision|BreakHitResult _outhit))
      (:then
        (return false))
      (:CastFailed
        _)))
  (return true))

(fn DroneRecharge
  (if (< (Variables|IncrementablePlayerStats|GetNumDrones) (Variables|IncrementablePlayerStats|GetDroneCapacity))
    (Math|Integer|IncrementInt (Variables|IncrementablePlayerStats|GetNumDrones)
      (:%20%20
        (if (< (Variables|IncrementablePlayerStats|GetNumDrones) (Variables|IncrementablePlayerStats|GetDroneCapacity))
          (return false)
          (else
            (return true)))))))

(fn CalculateandSetMaxSpeedandRange
  (Variables|IncrementablePlayerStats|SetMax%20Speed%20Level (Math|Float|Round (/ (- (Variables|IncrementablePlayerStats|GetMaxMovementSpeed) (Variables|IncrementablePlayerStats|GetMovementSpeed)) (Variables|IncrementValues|GetMovement%20Speed%20Increment%20Value))))
  (Variables|IncrementablePlayerStats|SetMax%20Range%20Level (Math|Float|Round (/ (- (Variables|IncrementablePlayerStats|GetMaxLazerRange) (Variables|IncrementablePlayerStats|GetLazerRange)) (Variables|IncrementValues|GetLazer%20Range%20Increment%20Value)))))

(fn LazerSpawn
  (return))