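; Player pawn or character for Beamerman that handles world-axis movement input and switching to a top-down camera.
; MoveForward drives world X and MoveRight drives world Y.
; When IsAxisLocked is set, IsMovingForward and IsMovingRight act as mutual locks, so the first axis pressed blocks the other and prevents diagonal movement.
; The SwitchCamera event sets player controller 0's view target to the supplied camera.
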(event Custom|SwitchCamera
  (params (TopDownCamera :type Camera%20Actor%20Object%20Reference))
  ;[1 1 1] Switch to top down camera
  (Game|Player|SetViewTargetwithBlend (Game|GetPlayerController 0) TopDownCamera 0.0 "VTBlend_Linear" 0.0 false))

(event Input|AxisEvents|InputAxisMoveForward
  (params (AxisValue :type Float%20%28single-precision%29))
  ;[1 1 1] Axis-locked Movement input
  (if (Variables|Default|GetisAxisLocked)
    (if (not (Variables|Default|GetisMovingRight))
      (if (!= AxisValue 0.0)
        (Variables|Default|SetisMovingForward true)
        (else
          (Variables|Default|SetisMovingForward false)))
      (Pawn|Input|AddMovementInput "1.000000,0.000000, 0" AxisValue false :!label _label))
    (else
      (goto _label))))

(event Input|AxisEvents|InputAxisMoveRight
  (params (AxisValue :type Float%20%28single-precision%29))
  ;[1 1 1] Axis-locked Movement input
  (if (Variables|Default|GetisAxisLocked)
    (if (not (Variables|Default|GetisMovingForward))
      (if (!= AxisValue 0.0)
        (Variables|Default|SetisMovingRight true)
        (else
          (Variables|Default|SetisMovingRight false)))
      (Pawn|Input|AddMovementInput "0.000000,1.000000, 0" AxisValue false :!label _label))
    (else
      (goto _label))))

(fn ConstructionScript)