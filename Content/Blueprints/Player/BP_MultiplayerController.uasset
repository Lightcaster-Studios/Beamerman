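; Player controller for Beamerman multiplayer matches that handles pawn allocation, match UI and the victory screen.
; AllocatePlayer spawns and possesses a pawn class per PlayerIndex at its PlayerStart, registering it with the game mode, though slots 2–3 register only placeholder entries.
; Events show countdown and HUD widgets, Enter triggers the game mode countdown, and victory pauses play to show GameState records.
; An appearance helper applies per-index meshes and materials but is never called here.
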(event Custom|ShowCountdown
  ;[1 1 1] Countdown
  (bind _returnvalue (UserInterface|CreateWidget "/Game/UI/HUD/CountdownWidget.CountdownWidget_C"))
  (UserInterface|Viewport|AddtoViewport _returnvalue 0))

(event Custom|Unfreeze
  ;[1 1 1] Countdown
  (Input|EnableInput (Pawn|GetControlledPawn) self))

(event Custom|Victory!
  ;[1 1 1] UI
  (Viewport|RemoveAllWidgets)
  (Game|SetGamePaused true)
  (Variables|/Script/Engine.PlayerController|SetbShowMouseCursor self true)
  (Input|DisableInput self)
  (bind _aspersistent_game_instance (Utilities|Casting|CastToPersistentGameInstance (Game|GetGameInstance)))
  (Default|PlayEndGameAudio _aspersistent_game_instance)
  (bind _asbp_multiplayer_game_state (Utilities|Casting|CastToBP_MultiplayerGameState (Game|GetGameState)))
  (bind _returnvalue (UserInterface|CreateWidget "/Game/UI/EndGameVictory/UI_Victory.UI_Victory_C" self (Variables|/Game/Blueprints/Player/BP_MultiplayerGameState.BP_MultiplayerGameState_C|GetPlayerRecords _asbp_multiplayer_game_state)))
  (bind _output_get (Variables|Default|SetVictoryWidgetRef _returnvalue))
  (Variables|/Game/UI/EndGameVictory/UI_Victory.UI_Victory_C|SetCurrentLevelName _output_get "LobbyMap")
  (UserInterface|Animation|PlayAnimation (Variables|Default|GetVictoryWidgetRef) (Variables|/Game/UI/EndGameVictory/UI_Victory.UI_Victory_C|GetSlide (Variables|Default|GetVictoryWidgetRef)) 0.0 1 "Forward" 1.0 false)
  (UserInterface|Viewport|AddtoViewport (Variables|Default|GetVictoryWidgetRef) 0))

(event Custom|OnlineMultiplayerGameHUD
  ;[1 1 1] UI
  (bind _returnvalue (UserInterface|CreateWidget "/Game/UI/HUD/OnlineMultiplayerGameWidgetHUD.OnlineMultiplayerGameWidgetHUD_C"))
  (UserInterface|Viewport|AddtoViewport _returnvalue 0))

(event EventBeginPlay
  ;[1 1 1] Create player indicator for each player
  (bind _asbp_beamerman_multi_player (Utilities|Casting|CastToBP_BeamermanMultiPlayer (Pawn|GetControlledPawn)))
  (Rendering|ToggleVisibility (Variables|/Game/Blueprints/Player/BP_BeamermanMultiPlayer.BP_BeamermanMultiPlayer_C|GetTextRender _asbp_beamerman_multi_player) false))

(event EventAllocatePlayer
  ;[1 1 1] Allocate Player
  (bind _outactors (Actor|GetAllActorsOfClass "/Script/Engine.PlayerStart"))
  (Variables|Default|SetPlayerStart _outactors)
  (switch int (Variables|Default|GetPlayerIndex)
    (:0
      (bind _returnvalue (Game|SpawnActorfromClass "/Game/Blueprints/Player/BP_Multiplayer_1.BP_Multiplayer_1_C" (Transformation|GetActorTransform (Utilities|Array|Get(acopy) (Variables|Default|GetPlayerStart))) "Undefined" 0 0 0))
      (Pawn|Possess _returnvalue)
      (bind _asbp_beamerman_multi_player (Utilities|Casting|CastToBP_BeamermanMultiPlayer (Pawn|GetControlledPawn)))
      (bind _output_get (Variables|/Game/Blueprints/Player/BP_BeamermanMultiPlayer.BP_BeamermanMultiPlayer_C|SetPlayerID _asbp_beamerman_multi_player (Variables|Default|GetPlayerIndex)))
      (bind _asbp_multiplayer_game_mode (Utilities|Casting|CastToBP_MultiplayerGameMode (Game|GetGameMode)))
      (Utilities|Map|Add (Variables|/Game/Blueprints/Player/BP_MultiplayerGameMode.BP_MultiplayerGameMode_C|GetPlayerIndexToPlayerRef _asbp_multiplayer_game_mode) _output_get _asbp_beamerman_multi_player))
    (:1
      (bind _returnvalue_2 (Game|SpawnActorfromClass "/Game/Blueprints/Player/BP_Multiplayer_2.BP_Multiplayer_2_C" (Transformation|GetActorTransform (Utilities|Array|Get(acopy) (Variables|Default|GetPlayerStart) 1)) "Undefined" 0 0 0))
      (Pawn|Possess _returnvalue_2)
      (bind _asbp_beamerman_multi_player_2 (Utilities|Casting|CastToBP_BeamermanMultiPlayer (Pawn|GetControlledPawn)))
      (bind _output_get_2 (Variables|/Game/Blueprints/Player/BP_BeamermanMultiPlayer.BP_BeamermanMultiPlayer_C|SetPlayerID _asbp_beamerman_multi_player_2 (Variables|Default|GetPlayerIndex)))
      (bind _asbp_multiplayer_game_mode_2 (Utilities|Casting|CastToBP_MultiplayerGameMode (Game|GetGameMode)))
      (Utilities|Map|Add (Variables|/Game/Blueprints/Player/BP_MultiplayerGameMode.BP_MultiplayerGameMode_C|GetPlayerIndexToPlayerRef _asbp_multiplayer_game_mode_2) _output_get_2 _asbp_beamerman_multi_player_2))
    (:2
      (bind _returnvalue_3 (Game|SpawnActorfromClass "/Game/Blueprints/Player/BP_Multiplayer_3.BP_Multiplayer_3_C" (Transformation|GetActorTransform (Utilities|Array|Get(acopy) (Variables|Default|GetPlayerStart) 2)) "Undefined" 0 0 0))
      (Pawn|Possess _returnvalue_3)
      (bind _asbp_beamerman_multi_player_3 (Utilities|Casting|CastToBP_BeamermanMultiPlayer (Pawn|GetControlledPawn)))
      (Variables|/Game/Blueprints/Player/BP_BeamermanMultiPlayer.BP_BeamermanMultiPlayer_C|SetPlayerID _asbp_beamerman_multi_player_3 (Variables|Default|GetPlayerIndex))
      (bind _asbp_multiplayer_game_mode_3 (Utilities|Casting|CastToBP_MultiplayerGameMode (Game|GetGameMode)))
      (Utilities|Map|Add (Variables|/Game/Blueprints/Player/BP_MultiplayerGameMode.BP_MultiplayerGameMode_C|GetPlayerIndexToPlayerRef _asbp_multiplayer_game_mode_3) 0 0))
    (:3
      (bind _returnvalue_4 (Game|SpawnActorfromClass "/Game/Blueprints/Player/BP_Multiplayer_4.BP_Multiplayer_4_C" (Transformation|GetActorTransform (Utilities|Array|Get(acopy) (Variables|Default|GetPlayerStart) 3)) "Undefined" 0 0 0))
      (Pawn|Possess _returnvalue_4)
      (bind _asbp_beamerman_multi_player_4 (Utilities|Casting|CastToBP_BeamermanMultiPlayer (Pawn|GetControlledPawn)))
      (Variables|/Game/Blueprints/Player/BP_BeamermanMultiPlayer.BP_BeamermanMultiPlayer_C|SetPlayerID _asbp_beamerman_multi_player_4 (Variables|Default|GetPlayerIndex))
      (bind _asbp_multiplayer_game_mode_4 (Utilities|Casting|CastToBP_MultiplayerGameMode (Game|GetGameMode)))
      (Utilities|Map|Add (Variables|/Game/Blueprints/Player/BP_MultiplayerGameMode.BP_MultiplayerGameMode_C|GetPlayerIndexToPlayerRef _asbp_multiplayer_game_mode_4) 0 0))))

(event Input|KeyboardEvents|Enter
  (params (Key :type Key%20Structure :default "None"))
  ;[1 1 1] Countdown
  (:Pressed
    (bind _asbp_multiplayer_game_mode (Utilities|Casting|CastToBP_MultiplayerGameMode (Game|GetGameMode)))
    (Default|Countdown _asbp_multiplayer_game_mode)))

(fn ConstructionScript)

(fn SetPlayerAppearance
  (params (PlayerIndex :type Integer) (Player :type BP%20Beamerman%20Multi%20Player%20Object%20Reference))
  (bind _mesh (Variables|/Script/Engine.Character|GetMesh Player))
  (Variables|/Game/Blueprints/Player/BP_BeamermanMultiPlayer.BP_BeamermanMultiPlayer_C|SetDroneMaterial Player (Utilities|Array|Get(acopy) (Variables|PlayerAppearance|GetPlayerDroneMaterials) PlayerIndex))
  (Variables|/Game/Blueprints/Player/BP_BeamermanMultiPlayer.BP_BeamermanMultiPlayer_C|SetLazerMaterial Player (Utilities|Array|Get(acopy) (Variables|PlayerAppearance|GetPlayerLazerMaterials) PlayerIndex))
  (Class|SkinnedMeshComponent|SetSkeletalMesh _mesh (Utilities|Array|Get(acopy) (Variables|PlayerAppearance|GetPlayerSkeletalMeshes) PlayerIndex) true)
  (Rendering|Material|SetMaterial _mesh 1 (Utilities|Array|Get(acopy) (Variables|PlayerAppearance|GetPlayerMaterials) PlayerIndex)))

(fn OnRepPlayerIndex)