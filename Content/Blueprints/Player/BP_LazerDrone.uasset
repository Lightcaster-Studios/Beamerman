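; Short-lived laser drone, owned and colored by a Beamerman player, that snaps to the grid and destroys itself shortly after spawning.
; FireWeapon plays a sound, waits out the charge time, then spawns a BP_LaserPulse along the arrow with reflect level and range.
; Per-player collision channels from PersistentGameInstance let the drone block players outside it at spawn, while overlapping players become blocked once they leave.
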(event OnComponentEndOverlap(DroneCollider)
  (params (OverlappedComponent :type Primitive%20Component%20Object%20Reference) (OtherActor :type Actor%20Object%20Reference) (OtherComp :type Primitive%20Component%20Object%20Reference) (OtherBodyIndex :type Integer))
  (bind _asbp_beamerman_player (Utilities|Casting|CastToBP_BeamermanPlayer OtherActor))
  (CallFunction|SetPlayerCollision _asbp_beamerman_player true))

(event Custom|FireWeapon
  (params (ReflectLevel :type Integer) (LazerRange :type Float%20%28single-precision%29) (ChargingTime :type Float%20%28single-precision%29))
  (bind _lazerspawnarrow (Variables|Default|GetLazerSpawnArrow))
  (bind _returnvalue (Transformation|GetWorldTransform _lazerspawnarrow))
  (CallFunction|PlayWeaponFireSFX)
  (Utilities|FlowControl|Delay ChargingTime)
  (bind _returnvalue_2 (Game|SpawnActorfromClass "/Game/Blueprints/Projectiles/BP_laserPulse.BP_LaserPulse_C" (Math|Transform|MakeTransform (.location _returnvalue) (.rotation _returnvalue) "1,1,1") "Undefined" self 0))
  (Default|SetLazerParams _returnvalue_2 ReflectLevel LazerRange (Math|Vector|GetForwardVector (Variables|Default|GetLazerSpawnArrow)))
  (Variables|Default|SetLazer%20Range LazerRange))

(event EventBeginPlay
  (CallFunction|SnaptoGrid)
  (CallFunction|SetupDroneBlocking)
  (Utilities|FlowControl|Delay 1.2)
  (CallFunction|DestroyDrone))

(fn ConstructionScript
  (bind _asbp_beamerman_player (Utilities|Casting|CastToBP_BeamermanPlayer (Components|GetOwner)))
  (Rendering|Material|SetMaterial (Variables|Default|GetDroneBody) 0 (Variables|/Game/Blueprints/Player/BP_BeamermanPlayer.BP_BeamermanPlayer_C|GetDroneMaterial _asbp_beamerman_player))
  (Rendering|Material|SetMaterial (Variables|Default|GetReactorCore) 0 (Variables|/Game/Blueprints/Player/BP_BeamermanPlayer.BP_BeamermanPlayer_C|GetLazerMaterial _asbp_beamerman_player)))

(fn SnaptoGrid
  (Transformation|SetActorLocation (Utilities|XYLocationtoNearest (Transformation|GetActorLocation self) 100) false false)
  (Transformation|SetActorRotation (Math|Rotator|MakeRotator 0.0 0.0 (.yaw (Utilities|RotatortoNearest (Transformation|GetActorRotation self) 90)))))

(fn PlayWeaponFireSFX
  (Audio|PlaySoundatLocation "/Game/Audio/SFX/LazerFire_Cue.LazerFire_Cue" (Transformation|GetActorLocation) "0, 0, 0" 1.0 1.0 0.0 0 0 0))

(fn DestroyDrone
  (Actor|DestroyActor))

(fn SetPlayerCollision
  (params (Player :type BP%20Beamerman%20Player%20Object%20Reference) (Block :type Boolean))
  (bind _collisiontype (CallFunction|GetPlayerCollisionType Player))
  (if Block
    (Collision|SetCollisionResponsetoChannel (Variables|Default|GetDroneCollider) _collisiontype "ECR_Block")
    (else
      (Collision|SetCollisionResponsetoChannel (Variables|Default|GetDroneCollider) _collisiontype "ECR_Overlap"))))

(fn SetupDroneBlocking
  (bind _dronecollider (Variables|Default|GetDroneCollider))
  (bind _outactors (Collision|ComponentOverlapActors _dronecollider (Transformation|GetWorldTransform _dronecollider) (Utilities|Array|MakeArray "ObjectTypeQuery7" "ObjectTypeQuery8" "ObjectTypeQuery9" "ObjectTypeQuery10") "/Game/Blueprints/Player/BP_BeamermanPlayer.BP_BeamermanPlayer_C"))
  (for _array_element _outactors
    (bind _asbp_beamerman_player (Utilities|Casting|CastToBP_BeamermanPlayer _array_element))
    (Utilities|Array|Add (LocalVariables|GetOverlappedPlayers) _asbp_beamerman_player))
  (bind _aspersistent_game_instance (Utilities|Casting|CastToPersistentGameInstance (Game|GetGameInstance)))
  (for _array_element_2 (Variables|/Game/PersistentGameInstance.PersistentGameInstance_C|GetAllPlayers _aspersistent_game_instance)
    (if (not (Utilities|Array|ContainsItem (LocalVariables|GetOverlappedPlayers) _array_element_2))
      (CallFunction|SetPlayerCollision _array_element_2 true))))

(fn GetPlayerCollisionType
  (params (Player :type BP%20Beamerman%20Player%20Object%20Reference))
  (bind _aspersistent_game_instance (Utilities|Casting|CastToPersistentGameInstance (Game|GetGameInstance)))
  (return (.Value (Utilities|Map|Find (Variables|/Game/PersistentGameInstance.PersistentGameInstance_C|GetPlayerCollisionMappings _aspersistent_game_instance) Player))))