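; Game mode for online Beamerman matches: registers joining players, runs the countdown and declares the last survivor the winner.
; PostLogin assigns player indices until the match starts; Countdown then creates score trackers, unfreezes players, starts the timer and shows HUDs.
; Each player capsule gets its own collision channel, stored in the game instance.
; Deaths record time and score; Tick detects one survivor and passes records to the game state.
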(event Custom|Countdown
  (if (not (Variables|Default|GetOnline%20Multiplayer%20Game%20Started?))
    (for _array_element (Variables|Default|GetPlayers)
      (Default|ShowCountdown _array_element)
      (Widget|RemovefromParent (stale EventBeginPlay _returnvalue)))
    (Variables|Default|SetOnline%20Multiplayer%20Game%20Started? true)
    (CallFunction|SetGameState)
    (CallFunction|CreateScore)
    (Utilities|FlowControl|Delay 3.0)
    (CallFunction|Unfreeze)
    (CallFunction|Collision)
    (CallFunction|GameHUD)))

(event Custom|Unfreeze
  ;[1 1 1] Unfreeze
  (for _array_element (Variables|Default|GetPlayers)
    (Default|Unfreeze _array_element))
  (Variables|/Game/Blueprints/Player/BP_MultiplayerGameState.BP_MultiplayerGameState_C|SetCurrentTime (Variables|Default|GetMyGameState) (Variables|Default|GetMatchTime))
  (Utilities|Time|SetTimerbyEvent (delegate Custom|Count) 1.0 true))

(event Custom|Count
  ;[1 1 1] Unfreeze
  (Math|Integer|DecrementInt (Variables|/Game/Blueprints/Player/BP_MultiplayerGameState.BP_MultiplayerGameState_C|GetCurrentTime (Variables|Default|GetMyGameState))))

(event Custom|Collision
  ;[1 1 1] Unfreeze
  (CallFunction|SetPlayerCollisions)
  (bind _aspersistent_game_instance (Utilities|Casting|CastToPersistentGameInstance (Game|GetGameInstance)))
  (Variables|/Game/PersistentGameInstance.PersistentGameInstance_C|SetAllOnlinePlayers _aspersistent_game_instance (Variables|Default|GetAllPlayers)))

(event Custom|GameHUD
  (for _array_element (Variables|Default|GetPlayers)
    (Default|OnlineMultiplayerGameHUD _array_element)))

(event Custom|Set%20Game%20State
  (bind _asbp_multiplayer_game_state (Utilities|Casting|CastToBP_MultiplayerGameState (Game|GetGameState)))
  (Variables|/Game/Blueprints/Player/BP_MultiplayerGameState.BP_MultiplayerGameState_C|SetPlayers _asbp_multiplayer_game_state (Variables|Default|GetAllPlayers)))

(event Custom|Victory
  ;[1 1 1] End Game
  (bind _result (Utilities|Set|ToArray (Variables|Default|GetAlivePlayers)))
  (CallFunction|AddPlayerRecord (.Value (Utilities|Map|Find (Variables|Default|GetPlayerIndexToPlayerRef) (Utilities|Array|Get(acopy) _result))))
  (bind _asbp_multiplayer_game_state (Utilities|Casting|CastToBP_MultiplayerGameState (Game|GetGameState)))
  (Variables|/Game/Blueprints/Player/BP_MultiplayerGameState.BP_MultiplayerGameState_C|SetPlayerRecords _asbp_multiplayer_game_state (Variables|Default|GetPlayerRecords))
  (Utilities|FlowControl|Delay 1.0)
  (for _array_element (Variables|Default|GetPlayers)
    (Default|Victory! _array_element)))

(event Custom|Register%20Dead%20Player
  (params (DeadPlayer :type BP%20Beamerman%20Multi%20Player%20Object%20Reference))
  ;[1 1 1] End Game
  (CallFunction|RegisterCharacterDeathHelper DeadPlayer))

(event Custom|Create%20Score
  (for _array_element (Variables|Default|GetAllPlayers)
    (Default|CreateScoreTracker _array_element)))

(event EventBeginPlay
  (bind _asbp_multiplayer_game_state (Utilities|Casting|CastToBP_MultiplayerGameState (Game|GetGameState)))
  (Variables|Default|SetMyGameState _asbp_multiplayer_game_state)
  ;[0.09399 0.3135 1] Before game starts, create waiting widget
  (bind _returnvalue (UserInterface|CreateWidget "/Game/UI/HUD/WaitingServerStart.WaitingServerStart_C"))
  (UserInterface|Viewport|AddtoViewport _returnvalue 0))

(event EventTick
  (params (DeltaSeconds :type Float%20%28single-precision%29))
  ;[1 1 1] End Game
  (if (Math|Boolean|ANDBoolean (Variables|Default|GetOnline%20Multiplayer%20Game%20Started?) (== (Utilities|Set|Length (Variables|Default|GetAlivePlayers)) 1) (Variables|Default|GetNotVictory))
    (Variables|Default|SetNotVictory false)
    (CallFunction|Victory)))

(event EventPostLogin
  (params (NewPlayer :type Player%20Controller%20Object%20Reference))
  (bind _clientindex (Variables|Default|GetClientIndex))
  ;[1 1 1] Login in
  (if (not (Variables|Default|GetOnline%20Multiplayer%20Game%20Started?))
    (bind _asbp_multiplayer_controller (Utilities|Casting|CastToBP_MultiplayerController NewPlayer))
    (Utilities|Array|Add (Variables|Default|GetPlayers) _asbp_multiplayer_controller)
    (bind _output_get (Variables|Default|SetCurrentPlayer _asbp_multiplayer_controller))
    (Variables|/Game/Blueprints/Player/BP_MultiplayerController.BP_MultiplayerController_C|SetPlayerIndex _output_get (Utilities|Select :Index (Variables|Default|GetClientIndex) :Option%200 0 :Option%201 1 :Option%202 2 :Option%203 3))
    (Class|BPIMultiplayer|AllocatePlayer(Message) _output_get)
    (bind _asbp_beamerman_multi_player (Utilities|Casting|CastToBP_BeamermanMultiPlayer (Pawn|GetControlledPawn (Variables|Default|GetCurrentPlayer))))
    (Utilities|Array|Add (Variables|Default|GetAllPlayers) _asbp_beamerman_multi_player)
    (Utilities|Set|Add (Variables|Default|GetAlivePlayers) _clientindex)
    (Math|Integer|IncrementInt _clientindex)))

(fn ConstructionScript)

(fn SetPlayerCollisions
  (for (_array_element _array_index) (Variables|Default|GetAllPlayers)
    (switch int _array_index
      (:0
        (Collision|SetCollisionObjectType (Variables|/Script/Engine.Character|GetCapsuleComponent _array_element) "ECC_GameTraceChannel1"))
      (:1
        (Collision|SetCollisionObjectType (Variables|/Script/Engine.Character|GetCapsuleComponent _array_element) "ECC_GameTraceChannel2"))
      (:2
        (Collision|SetCollisionObjectType (Variables|/Script/Engine.Character|GetCapsuleComponent _array_element) "ECC_GameTraceChannel3"))
      (:3
        (Collision|SetCollisionObjectType (Variables|/Script/Engine.Character|GetCapsuleComponent _array_element) "ECC_GameTraceChannel4"))))
  (bind _aspersistent_game_instance (Utilities|Casting|CastToPersistentGameInstance (Game|GetGameInstance)))
  (for (_array_element_2 _array_index_2) (Variables|Default|GetAllPlayers)
    (switch int _array_index_2
      (:0
        (Utilities|Map|Add (Variables|/Game/PersistentGameInstance.PersistentGameInstance_C|GetOnlinePlayerCollisionMappings _aspersistent_game_instance) _array_element_2 (Utilities|Enum|LiteralenumECollisionChannel "ECC_GameTraceChannel1")))
      (:1
        (Utilities|Map|Add (Variables|/Game/PersistentGameInstance.PersistentGameInstance_C|GetOnlinePlayerCollisionMappings _aspersistent_game_instance) _array_element_2 (Utilities|Enum|LiteralenumECollisionChannel "ECC_GameTraceChannel2")))
      (:2
        (Utilities|Map|Add (Variables|/Game/PersistentGameInstance.PersistentGameInstance_C|GetOnlinePlayerCollisionMappings _aspersistent_game_instance) _array_element_2 (Utilities|Enum|LiteralenumECollisionChannel "ECC_GameTraceChannel3")))
      (:3
        (Utilities|Map|Add (Variables|/Game/PersistentGameInstance.PersistentGameInstance_C|GetOnlinePlayerCollisionMappings _aspersistent_game_instance) _array_element_2 (Utilities|Enum|LiteralenumECollisionChannel "ECC_GameTraceChannel4"))))))

(fn RegisterCharacterDeathHelper
  (params (DeadPlayer :type BP%20Beamerman%20Multi%20Player%20Object%20Reference))
  (bind _output_get (Variables|Default|SetDeadPlayerRef DeadPlayer))
  (CallFunction|AddPlayerRecord _output_get)
  (Utilities|Set|Remove (Variables|Default|GetAlivePlayers) (Variables|/Game/Blueprints/Player/BP_BeamermanMultiPlayer.BP_BeamermanMultiPlayer_C|GetPlayerID (Variables|Default|GetDeadPlayerRef))))

(fn AddPlayerRecord
  (params (PlayerRef :type BP%20Beamerman%20Multi%20Player%20Object%20Reference))
  (bind _aspersistent_game_instance (Utilities|Casting|CastToPersistentGameInstance (Game|GetGameInstance)))
  (Utilities|Array|AddUnique (Variables|Default|GetPlayerRecords) (Utilities|Struct|MakeStruct_PlayerDeath (Variables|/Game/Blueprints/Player/BP_BeamermanMultiPlayer.BP_BeamermanMultiPlayer_C|GetPlayerID PlayerRef) (- 6e+01 (Variables|/Game/PersistentGameInstance.PersistentGameInstance_C|GetCurrentTimeRemaining _aspersistent_game_instance)) (Variables|/Game/Blueprints/Score/OnlineMultiplayerScoreTracker.OnlineMultiplayerScoreTracker_C|GetTotalScore (Variables|/Game/Blueprints/Player/BP_BeamermanMultiPlayer.BP_BeamermanMultiPlayer_C|GetScore%20Tracker PlayerRef))))
  (return))