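; AI controller for a bot that runs the AI_BT_Dodge behavior tree and feeds its Blackboard.
; AI Perception updates and per-tick line traces along four arrows sort targets by class into Drone, Player, PowerUp, BoxActor and Laser keys.
; Trace hits without a stimuli source are messaged to continue the trace, and ReverseTrace can store the reflector as the target.
; Control rotation snaps to 90-degree steps, and a dodge helper returns unblocked arrow directions.
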(event OnComponentDeactivated(AIPerception)
  (params (Component :type Actor%20Component%20Object%20Reference))
  (Development|PrintString (Utilities|GetDisplayName Component)))

(event OnTargetPerceptionUpdated(AIPerception)
  (params (Actor :type Actor%20Object%20Reference) (Stimulus :type AI%20Stimulus%20Structure))
  (CallFunction|SetBBValue Actor))

(event EventBeginPlay
  (AI|RunBehaviorTree "/Game/Blueprints/AIPlayer/AI_BT_Dodge.AI_BT_Dodge"))

(event EventTick
  (params (DeltaSeconds :type Float%20%28single-precision%29))
  (CallFunction|LockRotation)
  (CallFunction|RayTraceShoot (Variables|Default|GetFire%20Trace%20Range)))

(event EventReverseTrace
  (params (Actor :type Actor%20Object%20Reference) (Reflector :type Actor%20Object%20Reference))
  (if (== (Utilities|GetClass (Actor|GetComponentbyClass Actor "/Script/AIModule.AIPerceptionStimuliSourceComponent")) "/Script/AIModule.AIPerceptionStimuliSourceComponent")
    (CallFunction|SetRayTraceKey Actor Reflector)))

(fn ConstructionScript
  (Variables|Default|Setray%20trace%20direction (Utilities|Array|MakeArray (Variables|Default|GetArrow) (Variables|Default|GetArrow1) (Variables|Default|GetArrow2) (Variables|Default|GetArrow3))))

(fn RayTraceShoot
  (params (Trace%20Range :type Integer))
  (for _array_element (Variables|Default|Getray%20trace%20direction)
    (CallFunction|RayTracefromArrowandSetKey _array_element Trace%20Range)))

(fn RayTracefromArrowandSetKey
  (params (Arrow :type Arrow%20Component%20Object%20Reference) (range :type Integer))
  (bind _returnvalue (Transformation|GetWorldLocation Arrow))
  (bind _returnvalue_2 (Math|Vector|GetForwardVector Arrow))
  (bind (_outhit _returnvalue_3) (Collision|LineTraceByChannel _returnvalue (+ (* _returnvalue_2 range) _returnvalue) "TraceTypeQuery1" false 0 "None" true "(R=0.780625,G=0.000000,B=1.000000,A=1.000000)" "(R=0.000000,G=1.000000,B=0.000000,A=1.000000)" 0.5))
  (if _returnvalue_3
    (if (== (Utilities|GetClass (Actor|GetComponentbyClass (.HitActor (Collision|BreakHitResult _outhit)) "/Script/AIModule.AIPerceptionStimuliSourceComponent")) "/Script/AIModule.AIPerceptionStimuliSourceComponent")
      (CallFunction|SetRayTraceKey (.HitActor (Collision|BreakHitResult _outhit)))
      (else
        (Class|BPITraceable|TracefromIncidence(Message) (.HitActor (Collision|BreakHitResult _outhit)) _returnvalue_2 self)))))

(fn PrioritiseBlackBoardValue
  (params (Actors :type Array%20of%20Actor%20Object%20References))
  (Development|PrintString (Utilities|String|ToString(Integer) (Utilities|Array|Length Actors)) false)
  (bind _array_element (Utilities|Array|ForEachLoopwithBreak Actors :!label _label)
    (:LoopBody
      (if (== (Utilities|GetClass _array_element) "/Game/Blueprints/Player/BP_BeamermanPlayer.BP_BeamermanPlayer_C")
        (LocalVariables|SetClosest%20Object _array_element)
        (goto _label Break)
        (elif (or (Utilities|ClassIsChildOf (Utilities|GetClass _array_element) "/Game/Blueprints/Environment/Tiles/BP_CrateWall.BP_CrateWall_C") (Utilities|ClassIsChildOf (Utilities|GetClass _array_element) "/Game/Blueprints/PowerUps/BP_PowerUpDefault.BP_PowerUpDefault_C"))
          (Development|PrintString "find distance" false)
          (bind _distance (CallFunction|FindDistanceBetweenAI&Object _array_element))
          (if (< _distance (LocalVariables|Getshortest%20Distance))
            (LocalVariables|Setshortest%20Distance _distance)
            (LocalVariables|SetClosest%20Object _array_element))
          (else
            (Development|PrintString (Utilities|String|Append "Unknown class: " (Utilities|GetClassDisplayName (Utilities|GetClass _array_element))) false)))))
    (:Completed
      (CallFunction|SetBBValue (LocalVariables|GetClosest%20Object)))))

(fn LockRotation
  (Pawn|SetControlRotation (Utilities|RotatortoNearest 0 90)))

(fn SetBBValue
  (params (Actor :type Actor%20Object%20Reference) (Reflector :type Actor%20Object%20Reference))
  (bind _returnvalue (Utilities|GetClass Actor))
  (if (Utilities|Enum|Equal(Enum) (Utilities|String|ToString(Object) Reflector) "None") ; if ref == None, set actor as obj value\nelse, set ref as obj value
    (LocalVariables|SetObject%20Value Actor)
    (else
      (LocalVariables|SetObject%20Value Reflector)))
  (if (Utilities|ClassIsChildOf _returnvalue "/Game/Blueprints/Player/BP_LazerDrone.BP_LazerDrone_C")
    (AI|Components|Blackboard|SetValueasObject (Variables|Default|GetBlackboard) (Utilities|Name|MakeLiteralName "Drone") (LocalVariables|GetObject%20Value))
    (elif (Utilities|ClassIsChildOf _returnvalue "/Game/Blueprints/Player/BP_BeamermanPlayer.BP_BeamermanPlayer_C")
      (AI|Components|Blackboard|SetValueasObject (Variables|Default|GetBlackboard) (Utilities|Name|MakeLiteralName "Player") (LocalVariables|GetObject%20Value))
      (elif (Utilities|ClassIsChildOf _returnvalue "/Game/Blueprints/PowerUps/BP_PowerUpDefault.BP_PowerUpDefault_C")
        (AI|Components|Blackboard|SetValueasObject (Variables|Default|GetBlackboard) (Utilities|Name|MakeLiteralName "PowerUp") (LocalVariables|GetObject%20Value))
        (elif (Utilities|ClassIsChildOf _returnvalue "/Game/Blueprints/Environment/Tiles/BP_CrateWall.BP_CrateWall_C")
          (AI|Components|Blackboard|SetValueasObject (Variables|Default|GetBlackboard) (Utilities|Name|MakeLiteralName "BoxActor") (LocalVariables|GetObject%20Value))
          (elif (Utilities|ClassIsChildOf _returnvalue "/Game/Blueprints/Projectiles/BP_laserPulse.BP_LaserPulse_C")
            (AI|Components|Blackboard|SetValueasObject (Variables|Default|GetBlackboard) (Utilities|Name|MakeLiteralName "Laser") (LocalVariables|GetObject%20Value))
            (Development|PrintString "laser detected, set bb value as laser")
            (else
              (Development|PrintString "AI Stimuli not indicated"))))))))

(fn FindDistanceBetweenAI&Object
  (params (Actor :type Actor%20Object%20Reference))
  (return (Math|Vector|Distance(Vector) (Transformation|GetActorLocation Actor) (Transformation|GetWorldLocation (Variables|Default|GetScene)))))

(fn PrioritiseTargetforBB
  (params (Actor :type Actor%20Object%20Reference))
  (if (== (Utilities|GetClass Actor) "/Game/Blueprints/Player/BP_BeamermanPlayer.BP_BeamermanPlayer_C")
    (CallFunction|SetBBValue Actor)
    (else
      (bind _asactor (Utilities|Casting|CastToActor (AI|Components|Blackboard|GetValueasObject (Variables|Default|GetBlackboard) (Utilities|Name|MakeLiteralName "TargetInRadius")))
        (:CastFailed
          (CallFunction|SetBBValue Actor))))))

(fn SetRayTraceKey
  (params (Object%20Value :type Actor%20Object%20Reference) (Reflector :type Actor%20Object%20Reference))
  (if (Utilities|Enum|Equal(Enum) (Utilities|String|ToString(Object) Reflector) "None")
    (AI|Components|Blackboard|SetValueasObject (Variables|Default|GetBlackboard) (Utilities|Name|MakeLiteralName "RayTrace") Object%20Value)
    (CallFunction|SetBBValue Object%20Value Reflector)
    (else
      (AI|Components|Blackboard|SetValueasObject (Variables|Default|GetBlackboard) (Utilities|Name|MakeLiteralName "RayTrace") Reflector)
      (CallFunction|SetBBValue Object%20Value Reflector))))

(fn RayTraceDodgePaths
  (params (position :type Vector))
  (CallFunction|LockRotation)
  (for _array_element (Variables|Default|Getray%20trace%20direction)
    (bind _blocked (CallFunction|RayTracefromArrowforDodging _array_element (Variables|Default|GetDodge%20Trace%20Range) position))
    (if (not _blocked)
      (Utilities|Array|Add (LocalVariables|GetDirections) (Math|Vector|GetForwardVector _array_element))))
  (return (LocalVariables|GetDirections)))

(fn RayTracefromArrowforDodging
  (params (Arrow :type Arrow%20Component%20Object%20Reference) (range :type Integer) (Position :type Vector))
  (bind (_outhit _returnvalue) (Collision|LineTraceByChannel Position (+ (* (Math|Vector|GetForwardVector Arrow) range) Position) "TraceTypeQuery2" false 0 "None" true "(R=1.000000,G=0.000000,B=0.000000,A=1.000000)" "(R=0.000000,G=1.000000,B=0.000000,A=1.000000)" 0.5))
  (return _returnvalue))

(fn ShortestDistanceAssignKey
  (params (Key%20name :type Name) (Object :type Object%20Object%20Reference))
  (bind _blackboard (Variables|Default|GetBlackboard))
  (bind _asactor (Utilities|Casting|CastToActor Object)) ; actor from Object
  (bind _asactor_2 (Utilities|Casting|CastToActor (AI|Components|Blackboard|GetValueasObject _blackboard Key%20name)) ; actor from key
    (:then
      (if (< (Math|Vector|Distance(Vector) (Transformation|GetActorLocation _asactor) (Transformation|GetWorldLocation (Variables|Default|GetScene))) (Math|Vector|Distance(Vector) (Transformation|GetActorLocation _asactor_2) (Transformation|GetWorldLocation (Variables|Default|GetScene))))
        (AI|Components|Blackboard|SetValueasObject _blackboard Key%20name Object :!label _label)))
    (:CastFailed
      (goto _label))))